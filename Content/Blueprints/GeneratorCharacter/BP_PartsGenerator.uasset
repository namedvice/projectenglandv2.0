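; BP_PartsGenerator is an actor that resolves a modular character's mesh parts from a data table.
; Its Construction Script looks up CharacterRowName in DT_Parts and, if found, stores the head, body, pants, hands and boots meshes in variables.
; BeginPlay then clears the head, hands and body variables, leaving pants and boots set.
; The file does not show the meshes being applied to components.
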(event `self.ReceiveBeginPlay`
  (set `self.HeadMesh` null)
  (set `self.HandsMesh` null)
  (set `self.BodyMesh` null))

(fn `UserConstructionScript`
  (bind _returnvalue (`|GetDataTableRow` "/Game/Blueprints/GeneratorCharacter/DT_Parts.DT_Parts" (`self.CharacterRowName`))
    (:`then`
      (bind (_head _body _pants _boots _hands) (break `/Game/Blueprints/GeneratorCharacter/S_Parts` _returnvalue))
      (set `self.HeadMesh` _head)
      (set `self.BodyMesh` _body)
      (set `self.PantsMesh` _pants)
      (set `self.HandsMesh` _hands)
      (set `self.BootsMesh` _boots))))