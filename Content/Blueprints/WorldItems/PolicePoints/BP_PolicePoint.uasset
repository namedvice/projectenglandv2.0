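; BP_PolicePoint is a world spawn point that places a policeman when the player hero signals a police spawn.
; On BeginPlay it binds to the police-spawn event dispatcher on BP_BaseHero and unbinds after the first trigger.
; The spawn happens at the point's own transform, only while fewer than ten BP_Policeman actors exist in the world.
; The delayed random-timer respawn logic is disconnected, so each point spawns at most once.
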(event `self.ReceiveBeginPlay`
  (bind _asbp_base_hero (cast `/Game/Blueprints/Characters/BP_BaseHero` (`GameplayStatics.GetPlayerCharacter` 0)))
  (bind _output_get (set `self.Player` _asbp_base_hero))
  (add `/Game/Blueprints/Characters/BP_BaseHero.ED_PoliceSpawn` _output_get (delegate `StartSpawningPolicemen`))
  (`KismetSystemLibrary.PrintString` "Policemen on guard"))

(event `StartSpawningPolicemen`
  (`self.SpawnPolice`)
  (remove `/Game/Blueprints/Characters/BP_BaseHero.ED_PoliceSpawn` (`self.Player`) (delegate `StartSpawningPolicemen`)))

(event `SpawnPolice`
  (bind _outactors (`GameplayStatics.GetAllActorsOfClass` "/Game/ProjEng/Placeables/Characters/BP_Policeman.BP_Policeman_C"))
  (if (not (>= (`KismetArrayLibrary.Array_Length` _outactors) 10))
    (`|SpawnActorFromClass` "/Game/ProjEng/Placeables/Characters/BP_Policeman.BP_Policeman_C" (`self.GetTransform`) "AlwaysSpawn" "OverrideRootScale" null false null)))

(fn `UserConstructionScript`)