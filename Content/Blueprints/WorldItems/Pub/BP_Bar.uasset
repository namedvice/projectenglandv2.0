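; BP_Bar is the interactable pub bar that opens the pub menu when the player interacts with it.
; Interaction halts the player, plays a bartender greeting, and shows WB_PubMenu with a reference to the bar, cursor and UI-only input.
; Separate events toggle the Box collision to disable or re-enable interaction, with disabling also playing a bartender choice sound.
; BeginPlay caches all BP_FoodLocation actors in FoodLocations, which the bar's own graph does not otherwise use.
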(event `self.ReceiveBeginPlay`
  (`parent.ReceiveBeginPlay`)
  (bind _outactors (`GameplayStatics.GetAllActorsOfClass` "/Game/Blueprints/WorldItems/Pub/BP_FoodLocation.BP_FoodLocation_C"))
  (set `self.FoodLocations` _outactors))

(event `/Game/ProjEng/Data/Inventory/BPI_InventoryInteraction.OnInteract`
  (params (Actor :type "Actor Object Reference"))
  (bind _returnvalue (`GameplayStatics.GetPlayerController` 0))
  (set `PlayerController.bShowMouseCursor` true _returnvalue)
  (bind _returnvalue_2 (`|CreateWidget` "/Game/Blueprints/WorldItems/Pub/WB_PubMenu.WB_PubMenu_C" null self))
  (`UserWidget.AddToViewport` _returnvalue_2 0)
  (set `self.MenuWidget` _returnvalue_2)
  (`WidgetBlueprintLibrary.SetInputMode_UIOnlyEx` _returnvalue _returnvalue_2 "LockAlways")
  (`GameplayStatics.PlaySound2D` "/Game/ProjEng/Art/Sounds/Bartender/C_BartenderGreeting.C_BartenderGreeting" 1.0 1.0 0.0 null null)
  (`MovementComponent.StopMovementImmediately` (`Character.CharacterMovement` (`GameplayStatics.GetPlayerCharacter` 0))))

(event `DisableBarInteraction`
  (`PrimitiveComponent.SetCollisionEnabled` (`self.Box`) "NoCollision")
  (`GameplayStatics.PlaySound2D` "/Game/ProjEng/Art/Sounds/Bartender/C_BartenderChoice.C_BartenderChoice" 1.0 1.0 0.0 null null))

(event `EnableBarInteraction`
  (`PrimitiveComponent.SetCollisionEnabled` (`self.Box`) "QueryAndPhysics"))

(fn `UserConstructionScript`
  (`parent.UserConstructionScript`))