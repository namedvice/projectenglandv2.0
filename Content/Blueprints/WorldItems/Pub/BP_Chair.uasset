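; BP_Chair is an interactable chair that lets the player sit down and stand up on alternating interactions.
; It caches the BP_BaseHero player one second after BeginPlay, then a FlipFlop in OnInteract snaps them to the Sit or Stand point.
; Sitting plays a montage, sets IsSitting, disables movement and hides the interaction widget.
; Standing restores walking and clears IsSitting without animation, as the reversed montage is unwired.
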(event `self.ReceiveBeginPlay`
  (`parent.ReceiveBeginPlay`)
  (`KismetSystemLibrary.Delay` 1.0)
  (bind _asbp_base_hero (cast `/Game/ProjEng/Core/Characters/BP_BaseHero` (`GameplayStatics.GetPlayerCharacter` 0)))
  (set `self.As BP Base Hero` _asbp_base_hero))

(event `/Game/ProjEng/Data/Inventory/BPI_InventoryInteraction.OnInteract`
  (params (Actor :type "Actor Object Reference"))
  (bind _returnvalue (`GameplayStatics.GetPlayerCharacter` 0))
  (bind _returnvalue_2 (`GameplayStatics.GetPlayerCharacter` 0))
  (bind _sit (`self.Sit`))
  (bind _stand (`self.Stand`))
  (bind _as_bp_base_hero (`self.As BP Base Hero`))
  (`/Engine/EditorBlueprintResources/StandardMacros.FlipFlop`
    (:`A`
      (`self.K2_SetActorLocationAndRotation` _returnvalue_2 (`SceneComponent.K2_GetComponentLocation` _sit) (`SceneComponent.K2_GetComponentRotation` _sit) false false)
      (`|PlayMontage` (`Character.Mesh` _returnvalue_2) "/Game/ProjEng/Art/Characters/Worker/Animations/AM_Stand_To_Sit1.AM_Stand_To_Sit1"
        (:`then`
          (set `/Game/ProjEng/Core/Characters/BP_BaseHero.IsSitting?` true _as_bp_base_hero)
          (`CharacterMovementComponent.DisableMovement` (`Character.CharacterMovement` _returnvalue_2))
          (`SceneComponent.SetVisibility` (`self.WidgetInteraction`) false false))))
    (:`B`
      (`self.K2_SetActorLocationAndRotation` _returnvalue (`SceneComponent.K2_GetComponentLocation` _stand) (`SceneComponent.K2_GetComponentRotation` _stand) false false)
      (`CharacterMovementComponent.SetMovementMode` (`Character.CharacterMovement` _returnvalue) "MOVE_Walking" 0)
      (set `/Game/ProjEng/Core/Characters/BP_BaseHero.IsSitting?` false _as_bp_base_hero))))

(fn `UserConstructionScript`
  (`parent.UserConstructionScript`))