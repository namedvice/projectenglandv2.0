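; BP_Merchant is a merchant world actor that opens a merchant UI when the player interacts with it.
; OnInteract creates a WB_Merchant widget with a reference to itself on first use, caches it, and re-adds that instance to the viewport on later interactions.
; It then shows the mouse cursor, switches to Game and UI input focused on the widget, and disables player character input, with no restore logic in this Blueprint.
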(event `/Game/ProjEng/Data/Inventory/BPI_InventoryInteraction.OnInteract`
  (params (Actor :type "Actor Object Reference"))
  (bind _returnvalue (`GameplayStatics.GetPlayerController` 0))
  (bind _merchantwidget (`self.MerchantWidget`))
  (`/Engine/EditorBlueprintResources/StandardMacros.IsValid` _merchantwidget
    (:`Is Valid`
      (`UserWidget.AddToViewport` _merchantwidget 0))
    (:`Is Not Valid`
      (bind _returnvalue_2 (`|CreateWidget` "/Game/Blueprints/WorldItems/Pub/Merchant/WB_Merchant.WB_Merchant_C" null self))
      (bind _output_get (set `self.MerchantWidget` _returnvalue_2))
      (`UserWidget.AddToViewport` _output_get 0)))
  (set `PlayerController.bShowMouseCursor` true _returnvalue)
  (`WidgetBlueprintLibrary.SetInputMode_GameAndUIEx` _returnvalue (`self.MerchantWidget`) "DoNotLock" false)
  (`self.DisableInput` (`GameplayStatics.GetPlayerCharacter` 0) (`GameplayStatics.GetPlayerController` 0)))

(fn `UserConstructionScript`
  (`parent.UserConstructionScript`))