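; Interactable quest table where the player views mission briefings and plans and picks a mission.
; Interacting blends to a spawned, possessed table pawn with mouse input; Escape or P restores the character and destroys the pawn.
; Mission and submission child actors share a briefing widget, a timeline interpolates the plan widget, and the chosen level goes to ExitRef.
; UpdateSubmissions and HideSubmissions are empty, with some submission logic left disconnected.
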(event `Key|Escape`
  (params (Key :type "Key Structure"))
  (:`Pressed`
    (`self.ExitQuestTable` :!label _label)))

(event `Key|P`
  (params (Key :type "Key Structure"))
  (:`Pressed`
    (goto _label)))

(event `self.ReceiveBeginPlay`
  (bind _aswb_mission_briefing (cast `/Game/Blueprints/WorldItems/Pub/QuestTable/Mission/WB_MissionBriefing` (`WidgetComponent.GetWidget` (`self.MissionBriefing`)) :!pure true))
  (bind _aswb_mission_briefing_2 (cast `/Game/Blueprints/WorldItems/Pub/QuestTable/Mission/WB_MissionBriefing` (`WidgetComponent.GetWidget` (`self.MissionBriefing`)) :!pure true))
  (`parent.ReceiveBeginPlay`)
  (for _array_element (`|MakeArray` (`self.Mission1`))
    (bind _asbp_mission (cast `/Game/Blueprints/WorldItems/Pub/QuestTable/Mission/BP_Mission` (`ChildActorComponent.ChildActor` _array_element)))
    (set `/Game/Blueprints/WorldItems/Pub/QuestTable/Mission/BP_Mission.QuestTable` self _asbp_mission)
    (set `/Game/Blueprints/WorldItems/Pub/QuestTable/Mission/BP_Mission.NextTransform` (`SceneComponent.K2_GetComponentToWorld` (`self.BriefLocation`)) _asbp_mission)
    (set `/Game/Blueprints/WorldItems/Pub/QuestTable/Mission/BP_Mission.BriefingWidgetRef` _aswb_mission_briefing _asbp_mission)
    (set `/Game/Blueprints/WorldItems/Pub/QuestTable/Mission/WB_MissionBriefing.QuestTable` self _aswb_mission_briefing))
  (bind _output_get (set `self.Submissions` (`|MakeArray` (`self.Submission1`) (`self.Submission2`) (`self.Submission3`))))
  ;[1 1 1] For every submission set Mission Briefing Ref
  (for _array_element_2 _output_get
    (bind _asbp_sub_mission (cast `/Game/Blueprints/WorldItems/Pub/QuestTable/Mission/BP_SubMission` (`ChildActorComponent.ChildActor` _array_element_2)))
    (set `/Game/Blueprints/WorldItems/Pub/QuestTable/Mission/BP_Mission.BriefingWidgetRef` _aswb_mission_briefing_2 _asbp_sub_mission))
  ;[1 1 1] Hide Mission Briefing in the beginning
  (`Widget.SetVisibility` (`WidgetComponent.GetWidget` (`self.MissionBriefing`)) "Hidden")
  (`SceneComponent.K2_SetWorldLocation` (`self.Mission1`) (`SceneComponent.K2_GetComponentLocation` (`self.MissionLocation1`)) false false)
  (`UserWidget.SetOwningPlayer` _aswb_mission_briefing_2 (`GameplayStatics.GetPlayerController` 0)))

(event `/Game/ProjEng/Data/Inventory/BPI_InventoryInteraction.OnInteract`
  (params (Actor :type "Actor Object Reference"))
  (bind _returnvalue (`GameplayStatics.GetPlayerController` 0))
  (bind _returnvalue_2 (`GameplayStatics.GetPlayerCharacter` 0))
  ;[1 1 1] If player interacts with Quest Table - new Quest pawn spawns and gives player controll
  (`/Engine/EditorBlueprintResources/StandardMacros.DoOnce` false :!label _label_2
    (:`Completed`
      (`self.DisableInteraction`)
      (`self.EnableInput` (`GameplayStatics.GetPlayerController` 0))
      (bind _returnvalue_3 (`|SpawnActorFromClass` "/Game/Blueprints/WorldItems/Pub/QuestTable/BP_QuestTablePawn.BP_QuestTablePawn_C" (`self.GetTransform`) "AlwaysSpawn" "OverrideRootScale" null null))
      (bind _output_get (set `self.QuestPawn` _returnvalue_3))
      (`PlayerController.SetViewTargetWithBlend` (`GameplayStatics.GetPlayerController` 0) _output_get 1.5 "VTBlend_Cubic" 0.6 false)
      (set `MovementComponent.Velocity` (0.0 0.0 0.0) (`Character.CharacterMovement` _returnvalue_2))
      (set `self.SavedPlayerCharacter` _returnvalue_2)
      (`Controller.Possess` (`GameplayStatics.GetPlayerController` 0) _output_get)
      (`KismetSystemLibrary.Delay` 1.5)
      (set `PlayerController.bShowMouseCursor` true _returnvalue)
      (`WidgetBlueprintLibrary.SetInputMode_GameAndUIEx` _returnvalue (`WidgetComponent.GetWidget` (`self.MissionBriefing`)) "DoNotLock" false))))

(event `ExitQuestTable`
  (bind _returnvalue (`GameplayStatics.GetPlayerController` 0))
  ;[1 1 1] If player interacts with Quest Table - new Quest pawn spawns and gives player controll
  (`self.DisableInput` (`GameplayStatics.GetPlayerController` 0))
  (set `PlayerController.bShowMouseCursor` false _returnvalue)
  (`WidgetBlueprintLibrary.SetInputMode_GameOnly` _returnvalue)
  (`Controller.Possess` (`GameplayStatics.GetPlayerController` 0) (`self.SavedPlayerCharacter`))
  (bind _outactors (`GameplayStatics.GetAllActorsOfClass` "/Script/Engine.CameraActor"))
  (`PlayerController.SetViewTargetWithBlend` _returnvalue (`|GetArrayItem` _outactors 1) 1.5 "VTBlend_Cubic" 0.6 false)
  (`KismetSystemLibrary.Delay` 1.5)
  (`self.K2_DestroyActor` (`self.QuestPawn`))
  (`WidgetBlueprintLibrary.SetInputMode_GameOnly` (`GameplayStatics.GetPlayerController` 0))
  (`PrimitiveComponent.SetCollisionEnabled` (`self.Box`) "QueryOnly")
  (`PrimitiveComponent.SetCollisionEnabled` (`self.Sphere`) "QueryOnly")
  (goto _label_2 :!via `Reset`))

(event `UpdateSubmissions`
  ;[1 1 1] Update submissions with new ones
)

(event `ShowBriefing`
  ;[1 1 1] Briefing
  (`Widget.SetVisibility` (`WidgetComponent.GetWidget` (`self.MissionBriefing`)) "Visible")
  (`GameplayStatics.PlaySound2D` "/Game/Sounds/QuestTable/A_Button2.A_Button2" 1.0 1.0 0.0 null null))

(event `HideBriefing`
  ;[1 1 1] Briefing
  (`Widget.SetVisibility` (`WidgetComponent.GetWidget` (`self.MissionBriefing`)) "Hidden")
  (bind _asbp_mission (cast `/Game/Blueprints/WorldItems/Pub/QuestTable/Mission/BP_Mission` (`ChildActorComponent.ChildActor` (`self.Mission1`)))
    (:`then`
      (`/Game/Blueprints/WorldItems/Pub/QuestTable/Mission/BP_Mission.ResetInteraction` _asbp_mission))
    (:`CastFailed`
      (`KismetSystemLibrary.PrintString` "Hello"))))

(event `SetSubmissionsNextLocation`
  ;[1 1 1] When Player choose the Main Mission - set Submissions location to the right
  (for (_array_element _array_index) (`self.Submissions`)
    (bind (_returnvalue_location _returnvalue_rotation) (`KismetMathLibrary.BreakTransform` (`SceneComponent.K2_GetComponentToWorld` (`|GetArrayItem` (`|MakeArray` (`self.SubmissionShowingLocation1`) (`self.SubmissionShowingLocation2`) (`self.SubmissionShowingLocation3`)) _array_index))))
    (`self.K2_SetActorLocationAndRotation` (`ChildActorComponent.ChildActor` _array_element) _returnvalue_location _returnvalue_rotation false false)))

(event `HideSubmissions`
  ;[1 1 0] Hide Submissions
)

(event `OpenPlan`
  (bind _returnvalue (select `bool` (`self.bOpenPlan`) :`false` 0.03 :`true` 0.05))
  ;[1 1 0] Take Out/Hide Plan
  (`self.HideSubmissions`)
  (`GameplayStatics.PlaySound2D` "/Game/Sounds/QuestTable/A_Paper2.A_Paper2" 0.7 1.0 0.0 null null)
  (set `self.bOpenPlan` true)
  (bind _asbp_mission (cast `/Game/Blueprints/WorldItems/Pub/QuestTable/Mission/BP_Mission` (`ChildActorComponent.ChildActor` (`self.Mission1`))))
  (bind _planwidget (`/Game/Blueprints/WorldItems/Pub/QuestTable/Mission/BP_Mission.PlanWidget` _asbp_mission))
  (set `self.PlanWidgetDefaultLocation` (`SceneComponent.K2_GetComponentLocation` _planwidget))
  (`Timeline|Timeline_0_0` :!via `PlayFromStart` :!label _label_3
    (:`Update`
      (`SceneComponent.K2_SetRelativeLocation` _planwidget (`KismetMathLibrary.VInterpTo` (`SceneComponent.RelativeLocation` _planwidget) (select `bool` (`self.bOpenPlan`) :`true` (0.0 -90.0 5.0) :!type "Vector Structure") (`GameplayStatics.GetWorldDeltaSeconds`) 5.0) false false)
      (bind _planwidget_2 (`/Game/Blueprints/WorldItems/Pub/QuestTable/Mission/BP_Mission.PlanWidget` _asbp_mission))
      (bind (_returnvalue_x _returnvalue_y _returnvalue_z) (`KismetMathLibrary.BreakVector` (`SceneComponent.K2_GetComponentScale` _planwidget_2)))
      (`SceneComponent.SetWorldScale3D` _planwidget_2 (`KismetMathLibrary.VInterpTo` (`KismetMathLibrary.MakeVector` _returnvalue_x _returnvalue_y _returnvalue_z) (`KismetMathLibrary.MakeVector` _returnvalue_x _returnvalue _returnvalue) (`GameplayStatics.GetWorldDeltaSeconds`) 5.0)))))

(event `HidePlan`
  ;[1 1 0] Take Out/Hide Plan
  (`GameplayStatics.PlaySound2D` "/Game/Sounds/QuestTable/A_Button1.A_Button1" 1.0 1.0 0.0 null null)
  (set `self.bOpenPlan` false)
  (goto _label_3 :!via `PlayFromStart`))

(event `SetChosenMission`
  (params (ChosenLevelName :type Name) (bMissionAccepted :type Boolean))
  (bind _output_get (set `self.ChosenLevelName` ChosenLevelName))
  (set `self.bMissionAccepted` bMissionAccepted)
  (`/Game/Blueprints/WorldItems/Pub/QuestTable/BP_Exit.UpdateMissionInfo` (`self.ExitRef`) _output_get))

(fn `UserConstructionScript`
  (`parent.UserConstructionScript`))