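; BP_Exit is the Pub's exit trigger, which sends the player to the selected mission level.
; UpdateMissionInfo stores the level name, reveals a hidden cone marker and plays a timeline that drives the scene component's height.
; Player overlap with a mission set opens a gate and enters it after a short delay, calling GM_House's LoadLevel.
; Leaving the box closes the gate, so a brief touch does not trigger travel.
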(event `self.ReceiveBeginPlay`
  (`SceneComponent.SetVisibility` (`self.StaticMesh`) false false)
  (`SceneComponent.SetVisibility` (`self.Cone`) false false))

(event `self.Box.OnComponentBeginOverlap`
  (params (OverlappedComponent :type "PrimitiveComponent Object Reference") (OtherActor :type "Actor Object Reference") (OtherComp :type "PrimitiveComponent Object Reference") (OtherBodyIndex :type Integer) (bFromSweep :type Boolean) (SweepResult :type "HitResult Structure (by ref)"))
  (if (== OtherActor (`GameplayStatics.GetPlayerCharacter` 0))
    (if (!= (`self.MissionLevel`) "None")
      (`|ExecutionSequence`
        (:`then_0`
          (goto _label :!via `Open`))
        (:`then_1`
          (`KismetSystemLibrary.Delay` 0.2)
          (`/Engine/EditorBlueprintResources/StandardMacros.Gate` false :!label _label
            (:`Exit`
              (bind _asgm_house (cast `/Game/Blueprints/GameModes/GM_House` (`GameplayStatics.GetGameMode`)))
              (`/Game/Blueprints/GameModes/GM_House.LoadLevel` _asgm_house (`self.MissionLevel`) "Pub")))))
      (else
        (`KismetSystemLibrary.PrintString` "Mission None")))))

(event `self.Box.OnComponentEndOverlap`
  (params (OverlappedComponent :type "PrimitiveComponent Object Reference") (OtherActor :type "Actor Object Reference") (OtherComp :type "PrimitiveComponent Object Reference") (OtherBodyIndex :type Integer))
  (if (== OtherActor (`GameplayStatics.GetPlayerCharacter` 0))
    (goto _label :!via `Close`)))

(event `UpdateMissionInfo`
  (params (MissionLevel :type Name))
  (set `self.MissionLevel` MissionLevel)
  (`self.ShowMissionInfo`))

(event `ShowMissionInfo`
  (bind _scene (`self.Scene`))
  (bind (_relativelocation_x _relativelocation_y) (`KismetMathLibrary.BreakVector` (`SceneComponent.RelativeLocation` _scene)))
  (`SceneComponent.SetVisibility` (`self.StaticMesh`) true false)
  (`SceneComponent.SetVisibility` (`self.Cone`) true false)
  (bind (_direction _newtrack_0) (`Timeline|Timeline_0`)
    (:`Update`
      (`SceneComponent.K2_SetRelativeLocation` _scene (`KismetMathLibrary.MakeVector` _relativelocation_x _relativelocation_y (+ _newtrack_0 200.0)) false false))))

(fn `UserConstructionScript`)