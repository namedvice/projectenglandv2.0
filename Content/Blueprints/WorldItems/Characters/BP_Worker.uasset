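; BP_Worker is a character Blueprint for a worker who climbs walls, carries items and uses explosives.
; While hooking, W/S drive a timeline that moves the worker vertically, tracing for ground or ledge tops to resume walking.
; A looping timer keeps the PhysicsHandle target on the hand socket, and nearby actors form a cyclable highlight list.
; Hook detection, weapon dispatch and noise reporting are disconnected, and inventory and explosive functions are partly stubbed.
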(event `ChangeCamera`
  (params (Camera :type "CameraActor Object Reference")))

(event `self.ReceiveBeginPlay`
  ;[1 1 1] Begin Play
  (`parent.ReceiveBeginPlay`)
  (bind _asbp_main (cast `/Game/ProjEng/Core/Engine/BP_Main` (`GameplayStatics.GetPlayerController` 0))
    (:`then`
      (set `self.PC` _asbp_main))
    (:`CastFailed`
      (`KismetSystemLibrary.PrintString` "ControllerFailed"))))

(event `self.OnLanded`
  (params (Hit :type "HitResult Structure (by ref)"))
  ;[1 1 1] If there is space for hook up - hook up. If not - do nothing, cause it's too high
  (set `self.bCanClimb` true))

(event `Key|W`
  (params (Key :type "Key Structure"))
  (bind _returnvalue (`self.K2_GetActorLocation`))
  (bind _returnvalue_2 (`self.K2_GetActorLocation`))
  ;[1 1 1] Hooking Movement
  (:`Pressed`
    (if (`self.bHooking`)
      (bind _direction (`Timeline|Timeline_0_0` :!label _label)
        (:`Update`
          (switch `ETimelineDirection` _direction
            (:`Forward`
              (`self.K2_AddActorLocalOffset` (0.0 0.0 10.0)))
            (:`Backward`
              (`self.K2_AddActorLocalOffset` (0.0 0.0 -10.0))))
          (bind (_outhit _returnvalue_3) (`KismetSystemLibrary.LineTraceSingle` :`Start` _returnvalue :`End` (+ _returnvalue (* (`self.GetActorUpVector`) -50.0)) :`TraceChannel` "TraceTypeQuery1" :`DrawDebugType` "ForOneFrame"))
          (if _returnvalue_3
            (`self.Stop` :!label _label_2)
            (`CharacterMovementComponent.SetMovementMode` (`self.CharacterMovement`) "MOVE_Walking" 0)
            (set `self.bHooking` false)
            (set `self.bCanClimb` true)
            (else
              ;;[1 1 1] Climb Onto Surface
              (bind (_outhit_2 _returnvalue_4) (`KismetSystemLibrary.LineTraceSingle` :`Start` _returnvalue_2 :`End` (+ _returnvalue_2 (* (`self.GetActorForwardVector`) (`self.WallCheckLength`))) :`TraceChannel` "TraceTypeQuery1" :`DrawDebugType` "ForOneFrame"))
              (if (not _returnvalue_4)
                (`self.K2_AddActorLocalOffset` (60.0 0.0 50.0))
                (goto _label_2))))))))
  (:`Released`
    (goto _label :!via `Stop`)))

(event `Stop`
  ;[1 1 1] Hooking Movement
  (goto _label :!via `Stop`))

(event `Key|S`
  (params (Key :type "Key Structure"))
  ;[1 1 1] Hooking Movement
  (:`Pressed`
    (if (`self.bHooking`)
      (goto _label :!via `Reverse`)))
  (:`Released`
    (goto _label :!via `Stop`)))

(event `StopSetTargetLocationTimer`
  ;[1 1 1] Handle Item
  (`KismetSystemLibrary.K2_ClearAndInvalidateTimerHandle` (stale `TakeItem` _returnvalue)))

(event `TakeItem`
  (params (Component :type "PrimitiveComponent Object Reference"))
  ;[1 1 1] Handle Item
  (bind _output_get (set `self.GrabbedComponent` Component))
  (`PhysicsHandleComponent.GrabComponentAtLocation` (`self.PhysicsHandle`) _output_get "hand_r" (`SceneComponent.GetSocketLocation` Component "hand_r"))
  (bind _returnvalue (`KismetSystemLibrary.K2_SetTimerDelegate` (delegate `SetTargetLocation`) 0.01 true)))

(event `SetTargetLocation`
  ;[1 1 1] Handle Item
  (`PhysicsHandleComponent.SetTargetLocation` (`self.PhysicsHandle`) (`SceneComponent.GetSocketLocation` (`self.Mesh`) "hand_r")))

(event `Key|LeftMouseButton`
  (params (Key :type "Key Structure"))
  ;[1 1 1] Dynamite
)

(event `UpdateSplineComponents`
  (params (Points :type "Array of Vector Structure"))
  (bind _splinecomponents (`self.SplineComponents`))
  ;[1 1 1] Dynamite
  (for _array_element _splinecomponents
    (`ActorComponent.K2_DestroyComponent` _array_element))
  (`KismetArrayLibrary.Array_Clear` _splinecomponents)
  (for _array_element_2 Points
    (bind _returnvalue (`AddComponent|NODE_AddStaticMeshComponent-2` :`RelativeTransform` (`KismetMathLibrary.MakeTransform` (`KismetMathLibrary.InverseTransformLocation` (`self.GetTransform`) _array_element_2) (struct) (0.1 0.1 0.1))))
    (`SceneComponent.K2_SetWorldLocation` _returnvalue _array_element_2 false false)
    (`KismetArrayLibrary.Array_Add` (`self.SplineComponents`) _returnvalue)))

(fn `AddActorToClosest`
  (params (NewItem :type "Actor Object Reference (by ref)"))
  (bind _closestactors (`self.ClosestActors`))
  (bind _returnvalue (`KismetArrayLibrary.Array_Add` _closestactors NewItem))
  (if (== (`KismetArrayLibrary.Array_Length` _closestactors) 1)
    (set `self.CurrentItemIndex_0` _returnvalue)
    (set `self.HighlightedActor_0` NewItem)
    (else
      (return))))

(fn `AddToInventory`
  (params (NewItem :type "Name (by ref)")))

(fn `ChangeHighlightedActor`
  (if (== (`KismetArrayLibrary.Array_Length` (`self.ClosestActors`)) 0)
    (set `self.HighlightedActor_0` null)
    (set `self.CurrentItemIndex_0` 0)
    (else
      (bind _output_get (set `self.CurrentItemIndex_0` (+ (`self.CurrentItemIndex_0`) 1)))
      (if (>= _output_get (`KismetArrayLibrary.Array_Length` (`self.ClosestActors`)))
        (set `self.CurrentItemIndex_0` 0))
      (set `self.HighlightedActor_0` (`|GetArrayItem` (`self.ClosestActors`) (`self.CurrentItemIndex_0`)))))
  (return))

(fn `UpdateInventory`)

(fn `UserConstructionScript`
  (`parent.UserConstructionScript`))