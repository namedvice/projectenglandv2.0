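; BP_Drinker is a seated character that plays random idle animations and reacts when cheers happens.
; From BeginPlay it plays a random idle montage, re-rolling via a short timer on blend out.
; BindCheers subscribes it to the player BP_BaseHero's cheers dispatcher.
; On cheers it clears that timer, plays a random angry or clapping montage, then resumes the idle loop on completion.
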(event `self.ReceiveBeginPlay`
  (`|PlayMontage` (`self.Mesh`) (`KismetArrayLibrary.Array_Random` (`|MakeArray` "/Game/ProjEng/Art/Characters/Worker/Animations/AM_SittingLaughing.AM_SittingLaughing" "/Game/ProjEng/Art/Characters/Worker/Animations/AM_ThumbsUp.AM_ThumbsUp" "/Game/ProjEng/Art/Characters/Worker/Animations/AM_SittingStill.AM_SittingStill" :!type "AnimMontage Object Reference")) :!label _label
    (:`OnBlendOut`
      (bind _returnvalue (`KismetSystemLibrary.K2_SetTimerDelegate` (delegate `StartAnim`) 0.02)))))

(event `BindCheers`
  (bind _asbp_base_hero (cast `/Game/Blueprints/Characters/BP_BaseHero` (`GameplayStatics.GetPlayerCharacter` 0))
    (:`then`
      (add `/Game/Blueprints/Characters/BP_BaseHero.ED_Cheers` _asbp_base_hero (delegate `ED_Cheers_Event`)))
    (:`CastFailed`
      (`KismetSystemLibrary.PrintString` "Looser!"))))

(event `StartAnim`
  (goto _label))

(event `ED_Cheers_Event`
  (bind _mesh (`self.Mesh`))
  (`KismetSystemLibrary.K2_ClearAndInvalidateTimerHandle` (stale `self.ReceiveBeginPlay` _returnvalue))
  (`|PlayMontage` _mesh (`KismetArrayLibrary.Array_Random` (`|MakeArray` "/Game/ProjEng/Art/Characters/Worker/Animations/AM_StittingAngry.AM_StittingAngry" "/Game/ProjEng/Art/Characters/Worker/Animations/AM_Sitting_Clap_Montage.AM_Sitting_Clap_Montage" "/Game/ProjEng/Art/Characters/Worker/Animations/AM_Sitting_Clap__1__Montage.AM_Sitting_Clap__1__Montage" "/Game/ProjEng/Art/Characters/Worker/Animations/AM_Sitting_Clap__2__Montage.AM_Sitting_Clap__2__Montage" :!type "AnimMontage Object Reference"))
    (:`OnCompleted`
      (`SkeletalMeshComponent.Stop` _mesh)
      (goto _label))))

(fn `UserConstructionScript`)