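; BP_Drinker_Child2 is a character Blueprint, a child variant of a drinker character with a modular skeletal body.
; Its construction script runs the parent's, then sets the body, head, boots, hands and pants meshes to follow the main SkeletalMesh through master pose components.
; BeginPlay only defers to the parent, so any behavior comes from the parent class.
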(event `self.ReceiveBeginPlay`
  (`parent.ReceiveBeginPlay`))

(fn `UserConstructionScript`
  (`|ExecutionSequence`
    (:`then_0`
      (`parent.UserConstructionScript`))
    (:`then_1`
      (`SkinnedMeshComponent.SetLeaderPoseComponent` (`self.Body`) (`self.SkeletalMesh`) true)
      (`SkinnedMeshComponent.SetLeaderPoseComponent` (`self.Head`) (`self.SkeletalMesh`) true)
      (`SkinnedMeshComponent.SetLeaderPoseComponent` (`self.Boots`) (`self.SkeletalMesh`) true)
      (`SkinnedMeshComponent.SetLeaderPoseComponent` (`self.Hands`) (`self.SkeletalMesh`) true)
      (`SkinnedMeshComponent.SetLeaderPoseComponent` (`self.Pants`) (`self.SkeletalMesh`) true))))