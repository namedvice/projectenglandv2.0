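; BP_Jewelry is an interactable world item that yields loot and can set off a police response when damaged.
; After interaction it spawns a BP_Bag carrying its CurrencyAmount, disables further interaction and hides one mesh material slot with a transparent material.
; Its first damage event, gated by DoOnce, plays an explosion sound, makes another slot transparent and calls the police spawn dispatcher on the player's BP_BaseHero.
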(event `self.ReceiveBeginPlay`
  (`parent.ReceiveBeginPlay`))

(event `/Game/ProjEng/Data/Inventory/BPI_InventoryInteraction.OnInteract`
  (params (Actor :type "Actor Object Reference"))
  (`parent.OnInteract` Actor))

(event `self.PostInteraction`
  (`|SpawnActorFromClass` "/Game/ProjEng/Core/Bags/BP_Bag.BP_Bag_C" (`self.GetTransform`) "Undefined" "OverrideRootScale" null (`self.CurrencyAmount`) null)
  (`self.DisableInteraction`)
  (`PrimitiveComponent.SetMaterial` (`self.StaticMesh`) 3 "/Game/Blueprints/WorldItems/Jewelry/M_FullyTransparent.M_FullyTransparent"))

(event `self.ReceiveAnyDamage`
  (params (Damage :type "Float (single-precision)") (DamageType :type "DamageType Object Reference") (InstigatedBy :type "Controller Object Reference") (DamageCauser :type "Actor Object Reference"))
  (`/Engine/EditorBlueprintResources/StandardMacros.DoOnce` false
    (:`Completed`
      (`GameplayStatics.PlaySound2D` "/Game/GrenadePack/MapAssets/Audio/Explosion01.Explosion01" 1.0 1.0 0.0 null null)
      (`PrimitiveComponent.SetMaterial` (`self.StaticMesh`) 1 "/Game/Blueprints/WorldItems/Jewelry/M_FullyTransparent.M_FullyTransparent")
      (bind _asbp_base_hero (cast `/Game/Blueprints/Characters/BP_BaseHero` (`GameplayStatics.GetPlayerCharacter` 0)))
      (`/Game/Blueprints/Characters/BP_BaseHero.ED_PoliceSpawn` _asbp_base_hero))))

(fn `UserConstructionScript`)