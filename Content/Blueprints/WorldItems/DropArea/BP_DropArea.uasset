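; Getaway vehicle drop zone that banks loot bags and lets the player end the mission.
; Bags entering the box add their currency to GI_Main and are destroyed; a player still inside after a retriggerable delay triggers engine audio and GM_House's result widget.
; Arrive slides the mesh in on a delayed timeline and notifies of truck arrival, but its police-spawn binding, GMHouse setup and crate-collection logic are disconnected.
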(event `self.ReceiveBeginPlay`)

(event `Arrive`
  (bind _asbp_base_hero (cast `/Game/Blueprints/Characters/BP_BaseHero` (`GameplayStatics.GetPlayerCharacter` 0)))
  (remove `/Game/Blueprints/Characters/BP_BaseHero.ED_PoliceSpawn` _asbp_base_hero (delegate `Arrive`))
  (`KismetSystemLibrary.Delay` 30.0)
  (bind (_direction _newtrack_0) (`Timeline|Timeline_0`)
    (:`Update`
      (`SceneComponent.K2_SetRelativeLocation` (`self.StaticMesh`) (`KismetMathLibrary.MakeVector` _newtrack_0) false false))
    (:`Finished`
      (`/Game/UI/Notifiers/WB_Notifier.NewNotifier` (`/Game/Blueprints/GameModes/GM_House.NotifierWidget` (`self.GM_House`)) "TruckArrival"))))

(event `self.Box.OnComponentBeginOverlap`
  (params (OverlappedComponent :type "PrimitiveComponent Object Reference") (OtherActor :type "Actor Object Reference") (OtherComp :type "PrimitiveComponent Object Reference") (OtherBodyIndex :type Integer) (bFromSweep :type Boolean) (SweepResult :type "HitResult Structure (by ref)"))
  (bind _returnvalue (`GameplayStatics.GetPlayerCharacter` 0))
  (bind _asbp_bag (cast `/Game/ProjEng/Core/Bags/BP_Bag` OtherActor)
    (:`then`
      (bind _output_get (set `self.Bag` _asbp_bag))
      (bind _asgi_main (cast `/Game/ProjEng/Core/Engine/GI_Main` (`GameplayStatics.GetGameInstance`)))
      (`/Game/ProjEng/Core/Engine/GI_Main.AddAdditionalCurrency` _asgi_main (`/Game/ProjEng/Core/Bags/BP_Bag.CurrencyAmount` _output_get))
      (`/Game/ProjEng/Core/Interactables/BP_WorldItem.OnDrop` _output_get)
      (`self.K2_DestroyActor` _output_get))
    (:`CastFailed`
      (if (== OtherActor _returnvalue)
        (`KismetSystemLibrary.RetriggerableDelay` 2.0)
        ;[1 1 1] Mission Result
        (if (`PrimitiveComponent.IsOverlappingActor` (`self.Box`) _returnvalue)
          (`GameplayStatics.PlaySound2D` "/Game/Sounds/A_CarEngineStart.A_CarEngineStart" 1.0 1.0 0.0 null null)
          (bind _asgm_house (cast `/Game/Blueprints/GameModes/GM_House` (`GameplayStatics.GetGameMode`)))
          (`/Game/Blueprints/GameModes/GM_House.ShowResultWidget` _asgm_house true))))))

(fn `UserConstructionScript`)