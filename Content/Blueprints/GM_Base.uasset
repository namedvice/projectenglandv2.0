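; Base game mode that spawns and possesses the hero at a PlayerStart on BeginPlay and handles transitions between streamed levels.
; LoadLevel disables input, fades to black, unloads the current level and streams in the next.
; After fixed delays, it fades back in, moves the player to a found PlayerStart and restores input.
; Leaving the hardcoded "Store" level also destroys a BP_LevelTransition actor.
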(event `self.ReceiveBeginPlay`
  (bind _returnvalue (`GameplayStatics.GetActorOfClass` "/Script/Engine.PlayerStart"))
  (bind _returnvalue_2 (`|SpawnActorFromClass` "/Game/ProjEng/Core/Characters/BP_BaseHero_Child.BP_BaseHero_Child_C" (`self.GetTransform` _returnvalue) "AdjustIfPossibleButAlwaysSpawn" "OverrideRootScale" null null null))
  (`Controller.Possess` (`GameplayStatics.GetPlayerController` 0) _returnvalue_2))

(event `LoadLevel`
  (params (LevelName :type Name) (CurrentLevelName :type Name))
  ;[1 1 1] Load Level
  (`self.DisableInput` (`GameplayStatics.GetPlayerCharacter` 0) (`GameplayStatics.GetPlayerController` 0))
  (`PlayerCameraManager.StartCameraFade` :`self` (`GameplayStatics.GetPlayerCameraManager` 0) :`ToAlpha` 1.0 :`Duration` 1.0 :`bHoldWhenFinished` true)
  (`KismetSystemLibrary.Delay` 1.0)
  (bind _output_get (set `self.PreviousLevelName` CurrentLevelName))
  (`GameplayStatics.UnloadStreamLevel` _output_get)
  (`GameplayStatics.LoadStreamLevel` LevelName true)
  (`KismetSystemLibrary.Delay` 1.0)
  (`PlayerCameraManager.StartCameraFade` :`self` (`GameplayStatics.GetPlayerCameraManager` 0) :`FromAlpha` 1.0 :`Duration` 1.0)
  (bind _returnvalue (`GameplayStatics.GetActorOfClass` "/Script/Engine.PlayerStart"))
  (`self.K2_SetActorTransform` (`GameplayStatics.GetPlayerCharacter` 0) (`self.GetTransform` _returnvalue) false false)
  (`self.EnableInput` (`GameplayStatics.GetPlayerCharacter` 0) (`GameplayStatics.GetPlayerController` 0))
  ;[0.9016 1 0] Specify the Store level Name!!!
  (if (== (`self.PreviousLevelName`) "Store")
    (bind _returnvalue_2 (`GameplayStatics.GetActorOfClass` "/Game/Blueprints/WorldItems/LevelsTransition/BP_LevelTransition.BP_LevelTransition_C"))
    (`self.K2_DestroyActor` _returnvalue_2)))

(fn `UserConstructionScript`)