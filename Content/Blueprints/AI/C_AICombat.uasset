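; AI controller for combat enemies that runs a supplied behavior tree and stores the hero actor in its blackboard.
; Perception updates for the player character set CanSeePlayer from the first sensed stimulus, though any further stimulus entry clears it.
; Events toggle the Available input flag, and OnKill stops brain logic, sight and tick.
; Hearing, dead-ally, action-point, attack and closest-enemy targeting logic remains but is disconnected.
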(event `self.ReceiveBeginPlay`)

(event `RunBehaviourTree`
  (params (BTAsset :type "BehaviorTree Object Reference"))
  (`self.RunBehaviorTree` BTAsset)
  (bind _returnvalue (`GameplayStatics.GetActorOfClass` "/Game/Blueprints/Characters/BP_BaseHero.BP_BaseHero_C"))
  (`BlackboardComponent.SetValueAsObject` (`AIBlueprintHelperLibrary.GetBlackboard` null) "CurrentHero" _returnvalue))

(event `UnlockInput`
  (`BlackboardComponent.SetValueAsBool` (`AIBlueprintHelperLibrary.GetBlackboard` null) "Available" true))

(event `BlockInput`
  (`BlackboardComponent.SetValueAsBool` (`AIBlueprintHelperLibrary.GetBlackboard` null) "Available" false))

(event `self.AIPerception.OnPerceptionUpdated`
  (params (UpdatedActors :type "Array of Actor Object Reference (by ref)"))
  (bind (_localsense_age _localsense_expirationage _localsense_strength _localsense_stimuluslocation _localsense_receiverlocation _localsense_tag _localsense_bsuccessfullysensed) (break `AIStimulus` (`self.LocalSense`)))
  (bind _output_get (set `self.Updated Actors` UpdatedActors))
  (for _array_element _output_get
    (bind _info (`AIPerceptionComponent.GetActorsPerception` (`self.AIPerception`) _array_element))
    (bind _output_get_2 (set `self.SensedActor` (break `ActorPerceptionBlueprintInfo` _info)))
    (if (== _output_get_2 (`GameplayStatics.GetPlayerCharacter` 0))
      (for (_array_element_2 _array_index) (`.LastSensedStimuli` (break `ActorPerceptionBlueprintInfo` _info))
        (set `self.LocalSense` _array_element_2)
        (switch `int` _array_index
          (:`Default`
            (`self.LostPlayer`))
          (:`0`
            (if _localsense_bsuccessfullysensed
              (`self.SeenPlayer`)
              (else
                (`self.LostPlayer`)))))))))

(event `SeenPlayer`
  (`BlackboardComponent.SetValueAsBool` (`AIBlueprintHelperLibrary.GetBlackboard` null) "CanSeePlayer" true))

(event `LostPlayer`
  (`BlackboardComponent.SetValueAsBool` (`AIBlueprintHelperLibrary.GetBlackboard` null) "CanSeePlayer" false))

(event `OnKill`
  (`BrainComponent.StopLogic` (`self.BrainComponent`) "Died")
  (`AIPerceptionComponent.SetSenseEnabled` (`self.AIPerception`) "/Script/AIModule.AISense_Sight" false)
  (`self.SetActorTickEnabled` false))

(event `self.ReceiveTick`
  (params (DeltaSeconds :type "Float (single-precision)")))

(fn `GetClosestEnemy`
  (params (Array :type "Array of Actor Object Reference"))
  (returns (ClosestEnemyActor :type "Actor Object Reference") (Success :type Boolean))
  (locals (ClosestDistance :type "Float (double-precision)" :default 1000000.0) (ClosestEnemy :type "Actor Object Reference"))
  (bind _closestenemy (`local.ClosestEnemy`))
  (bind _closestenemy_2 (`local.ClosestEnemy`))
  (bind _returnvalue (`self.GetDistanceTo` (`self.ControlledPawn`) _closestenemy))
  (set `local.ClosestEnemy` null)
  (for _array_element Array
    (if (not (`self.ActorHasTag` _array_element (`self.FriendAITag`)))
      (`/Engine/EditorBlueprintResources/StandardMacros.IsValid` _closestenemy
        (:`Is Valid`
          (if (< _returnvalue (`local.ClosestDistance`))
            (set `local.ClosestDistance` _returnvalue :!label _label)
            (set `local.ClosestEnemy` _array_element)))
        (:`Is Not Valid`
          (goto _label)))))
  (return _closestenemy_2 (`KismetSystemLibrary.IsValid` _closestenemy_2)))

(fn `UserConstructionScript`)