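; AI controller for stealth enemies that starts BT_AI and seeds its blackboard with wait time and the pawn's ActionPoint target and action.
; Custom events toggle the Available and CanSeePlayer keys.
; Helpers pick the closest non-friend actor as FocusedActor and update sight state.
; The perception handler is empty: logic for distance-curve sight detection, hearing investigation and dead-ally alerts is present but disconnected, so it never runs.
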(event `self.ReceiveBeginPlay`
  (bind _returnvalue (`AIBlueprintHelperLibrary.GetBlackboard` null))
  (`KismetSystemLibrary.Delay` 0.2)
  (`self.RunBehaviorTree` "/Game/Blueprints/AI/BT_AI.BT_AI")
  (`BlackboardComponent.SetValueAsFloat` (`AIBlueprintHelperLibrary.GetBlackboard` null) "WaitTime" 2.0)
  (bind _asbp_base_enemy (cast `/Game/Blueprints/Characters/BP_BaseEnemy` (`self.K2_GetPawn`)))
  (bind _output_get (set `self.ControlledPawn` _asbp_base_enemy))
  (bind _actionpoint (`/Game/Blueprints/Characters/BP_BaseEnemy.ActionPoint` _output_get))
  (`/Engine/EditorBlueprintResources/StandardMacros.IsValid` _actionpoint
    (:`Is Valid`
      (`BlackboardComponent.SetValueAsObject` _returnvalue "ActionPoint" _actionpoint)
      (bind _actioninfo_actiontomake (break `/Game/Blueprints/AI/ActionPoints/SActionInfo` (`/Game/Blueprints/AI/ActionPoints/BP_ActionPoint.ActionInfo` _actionpoint)))
      (`BlackboardComponent.SetValueAsEnum` _returnvalue "ActionStatus" _actioninfo_actiontomake)
      (`BlackboardComponent.SetValueAsVector` _returnvalue "TargetLocation" (`self.K2_GetActorLocation` _actionpoint)))))

(event `RunBehaviourTree`
  (params (BTAsset :type "BehaviorTree Object Reference")))

(event `UnlockInput`
  (`BlackboardComponent.SetValueAsBool` (`AIBlueprintHelperLibrary.GetBlackboard` null) "Available" true))

(event `BlockInput`
  (`BlackboardComponent.SetValueAsBool` (`AIBlueprintHelperLibrary.GetBlackboard` null) "Available" false))

(event `self.AIPerception.OnPerceptionUpdated`
  (params (UpdatedActors :type "Array of Actor Object Reference (by ref)")))

(event `SeenPlayer`
  (`BlackboardComponent.SetValueAsBool` (`AIBlueprintHelperLibrary.GetBlackboard` null) "CanSeePlayer" true))

(event `LostPlayer`
  (`BlackboardComponent.SetValueAsBool` (`AIBlueprintHelperLibrary.GetBlackboard` null) "CanSeePlayer" false))

(event `self.ReceiveTick`
  (params (DeltaSeconds :type "Float (single-precision)")))

(fn `GetClosestEnemy`
  (params (Array :type "Array of Actor Object Reference"))
  (returns (ClosestEnemyActor :type "Actor Object Reference") (Success :type Boolean))
  (locals (ClosestDistance :type "Float (double-precision)" :default 1000000.0) (ClosestEnemy :type "Actor Object Reference"))
  (bind _closestenemy (`local.ClosestEnemy`))
  (bind _closestenemy_2 (`local.ClosestEnemy`))
  (bind _returnvalue (`self.GetDistanceTo` (`self.ControlledPawn`) _closestenemy))
  (set `local.ClosestEnemy` null)
  (for _array_element Array
    (if (not (`self.ActorHasTag` _array_element (`self.FriendAITag`)))
      (`/Engine/EditorBlueprintResources/StandardMacros.IsValid` _closestenemy
        (:`Is Valid`
          (if (< _returnvalue (`local.ClosestDistance`))
            (set `local.ClosestDistance` _returnvalue :!label _label)
            (set `local.ClosestEnemy` _array_element)))
        (:`Is Not Valid`
          (goto _label)))))
  (return _closestenemy_2 (`KismetSystemLibrary.IsValid` _closestenemy_2)))

(fn `UserConstructionScript`)