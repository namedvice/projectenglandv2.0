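; BP_Porter is an AI character that can be set to follow the player and make a close-range attack.
; After a short delay on BeginPlay, it registers a callback with the player's BP_BaseHero via AssignEDPoliceSpawn, which sets the CanSeePlayer blackboard key when fired.
; Close attacks play a throw montage and apply delayed, fixed damage straight to the player without a hit check.
; Distance attacks only print a placeholder message.
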(event `self.ReceiveBeginPlay`
  (`parent.ReceiveBeginPlay`)
  (`KismetSystemLibrary.Delay` 0.2)
  (bind _asbp_base_hero (cast `/Game/Blueprints/Characters/BP_BaseHero` (`GameplayStatics.GetPlayerCharacter` 0)))
  (add `/Game/Blueprints/Characters/BP_BaseHero.ED_PoliceSpawn` _asbp_base_hero (delegate `StartFollowingPlayer`)))

(event `StartFollowingPlayer`
  (`BlackboardComponent.SetValueAsBool` (`AIBlueprintHelperLibrary.GetBlackboard` (`AIBlueprintHelperLibrary.GetAIController` self)) "CanSeePlayer" true))

(event `/Game/Blueprints/AI/BPI_Enemy.Attack`
  (params (FocusedActor :type "Actor Object Reference") (bCloseAttack :type Boolean))
  (if bCloseAttack
    (`|PlayMontage` (`self.Mesh`) "/Game/ProjEng/Art/Characters/Worker/Animations/AM_Throw_AI.AM_Throw_AI"
      (:`then`
        (`KismetSystemLibrary.Delay` 0.5)
        (`GameplayStatics.ApplyDamage` (`GameplayStatics.GetPlayerCharacter` 0) 20.0)))
    (else
      (`KismetSystemLibrary.PrintString` "No distance attack"))))

(fn `UserConstructionScript`
  (`parent.UserConstructionScript`))