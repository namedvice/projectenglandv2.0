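; BP_BaseEnemy is a base enemy character with AI team tagging, sight-detection and health widgets, and selectable movement speeds.
; Highlighting briefly enables custom depth through a retriggerable delay, while looping timers re-register it as a sight stimulus or yaw it toward the player.
; Death unpossesses and ragdolls the enemy, reports the kill to GM_House, notifies the combat controller if the cast succeeds, then destroys the actor after a delay.
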(event `self.ReceiveBeginPlay`
  (`parent.ReceiveBeginPlay`)
  (`self.SetTeamTag`)
  (set `/Game/Blueprints/AI/AISight/WB_SightDetection.PawnOwner` self (cast `/Game/Blueprints/AI/AISight/WB_SightDetection` (`WidgetComponent.GetUserWidgetObject` (`self.SightDetection`)) :!pure true))
  (bind _aswb_health (cast `/Game/UI/Health/WB_Health` (`WidgetComponent.GetWidget` (`self.HealthWidget`))))
  (set `/Game/UI/Health/WB_Health.Character` self _aswb_health))

(event `StartPingTimer`
  (`KismetSystemLibrary.K2_SetTimerDelegate` (delegate `PingYourself`) 0.1 true))

(event `SetTeamTag`
  (bind _tags (`self.Tags`))
  (bind _returnvalue (`KismetArrayLibrary.Array_Find` _tags (`self.AITag`)))
  ;[1 1 1] Teams
  (bind _asc_aistealth (cast `/Game/Blueprints/AI/C_AIStealth` (`AIBlueprintHelperLibrary.GetAIController` self)))
  (if (> _returnvalue -1)
    (set `/Game/Blueprints/AI/C_AIStealth.FriendAITag` (`|GetArrayItem` _tags _returnvalue) _asc_aistealth)))

(event `Highlight`
  (bind _mesh (`self.Mesh`))
  (`PrimitiveComponent.SetRenderCustomDepth` _mesh true)
  (`KismetSystemLibrary.RetriggerableDelay` 0.1)
  (`PrimitiveComponent.SetRenderCustomDepth` _mesh false :!label _label))

(event `PingYourself`
  (`AIPerceptionStimuliSourceComponent.RegisterForSense` (`self.AIPerceptionStimuliSource_0`) "/Script/AIModule.AISense_Sight"))

(event `StopHighlight`
  (goto _label))

(event `SetAISpeed`
  (params (Speed :type "/Game/Blueprints/AI/EAISpeed Enum" :default "NewEnumerator0"))
  ;[1 1 1] Set AI Speed
  (set `CharacterMovementComponent.MaxWalkSpeed` (select `/Game/Blueprints/AI/EAISpeed` Speed :`NewEnumerator0` 300.0 :`NewEnumerator1` 600.0 :`NewEnumerator2` 100.0) (`self.CharacterMovement`)))

(event `Death`
  ;[1 1 1] Death
  (`ActorComponent.K2_DestroyComponent` (`self.HealthWidget`))
  (`Controller.UnPossess` (`self.GetController`))
  (`PrimitiveComponent.SetSimulatePhysics` (`self.Mesh`) true)
  (`MovementComponent.StopMovementImmediately` (`self.CharacterMovement`))
  (`PrimitiveComponent.SetCollisionEnabled` (`self.CapsuleComponent`) "NoCollision")
  (set `self.Dead` true)
  (bind _asgm_house (cast `/Game/Blueprints/GameModes/GM_House` (`GameplayStatics.GetGameMode`)))
  (`/Game/Blueprints/GameModes/GM_House.CountKilledEnemies` _asgm_house)
  (bind _asc_aicombat (cast `/Game/Blueprints/AI/C_AICombat` (`AIBlueprintHelperLibrary.GetAIController` self)))
  (`/Game/Blueprints/AI/C_AICombat.OnKill` _asc_aicombat)
  (`Controller.UnPossess` _asc_aicombat)
  (`KismetSystemLibrary.Delay` 7.0)
  (`self.K2_DestroyActor`))

(event `StartFacingPlayerTimer`
  (bind _returnvalue (`KismetSystemLibrary.K2_SetTimerDelegate` (delegate `FacePlayer`) 0.05 true)))

(event `StopFacingPlayerTimer`
  (`KismetSystemLibrary.K2_ClearAndInvalidateTimerHandle` (stale `StartFacingPlayerTimer` _returnvalue)))

(event `FacePlayer`
  (bind (_returnvalue_roll _returnvalue_pitch _returnvalue_yaw) (`KismetMathLibrary.BreakRotator` (`KismetMathLibrary.FindLookAtRotation` (`self.K2_GetActorLocation`) (`self.K2_GetActorLocation` (`GameplayStatics.GetPlayerCharacter` 0)))))
  (`self.K2_SetActorRotation` (`KismetMathLibrary.MakeRotator` 0.0 0.0 _returnvalue_yaw)))

(fn `UserConstructionScript`
  (`parent.UserConstructionScript`))