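; BP_BaseHero_Child is a hero character Blueprint, apparently derived from a base hero, with a body built from modular mesh parts.
; Its Construction Script runs the parent's script, then sets Mesh as the master pose component for Pants, Body, Head, Boots and Hands so they follow one skeleton pose.
; The event graph holds only disabled placeholder events, so it adds no gameplay logic of its own.
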(fn `UserConstructionScript`
  (`|ExecutionSequence`
    (:`then_0`
      (`parent.UserConstructionScript`))
    (:`then_1`
      (`SkinnedMeshComponent.SetLeaderPoseComponent` (`self.Pants`) (`self.Mesh`) true)
      (`SkinnedMeshComponent.SetLeaderPoseComponent` (`self.Body`) (`self.Mesh`) true)
      (`SkinnedMeshComponent.SetLeaderPoseComponent` (`self.Head`) (`self.Mesh`) true)
      (`SkinnedMeshComponent.SetLeaderPoseComponent` (`self.Boots`) (`self.Mesh`) true)
      (`SkinnedMeshComponent.SetLeaderPoseComponent` (`self.Hands`) (`self.Mesh`) true))))