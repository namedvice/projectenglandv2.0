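; Policeman AI character that spawns armed and attacks the player with a gun or pistol whip.
; On BeginPlay it binds its health widget, flags the player as seen, runs the policemen behaviour tree, and spawns a weapon from the items DataTable onto its hand socket.
; Attack either plays a pistol-whip montage with direct damage to the player or briefly fires the weapon.
; Death drops the weapon.
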(event `self.ReceiveBeginPlay`
  (`parent.ReceiveBeginPlay`)
  (bind _aswb_health (cast `/Game/UI/Health/WB_Health` (`WidgetComponent.GetWidget` (`self.HealthWidget`))))
  (set `/Game/UI/Health/WB_Health.Character` self _aswb_health)
  (bind _asc_aicombat (cast `/Game/Blueprints/AI/C_AICombat` (`AIBlueprintHelperLibrary.GetAIController` self)))
  (set `/Game/Blueprints/AI/C_AICombat.HaveSeenPlayer` true _asc_aicombat)
  (`/Game/Blueprints/AI/C_AICombat.RunBehaviourTree` _asc_aicombat "/Game/Blueprints/AI/BT_Policemen.BT_Policemen")
  (bind _returnvalue (`|GetDataTableRow` "/Game/ProjEng/Data/Inventory/DataTables/DT_Items.DT_Items" (`self.WeaponName`))
    (:`then`
      (bind ((`Price_44_BA17BE7C4ECB02FA107A0797172B8F9E` _price) (`Class_21_90F28F704DAD91E466A95D86CE2FF6E6` _class)) (break `/Game/ProjEng/Data/Inventory/Structures/SItemData` _returnvalue))
      (if (`KismetSystemLibrary.IsValidClass` _class)
        (bind _returnvalue_2 (`|SpawnActorFromClass` _class (`SceneComponent.GetSocketTransform` (`self.Mesh`) "weapon" "RTS_World") "AlwaysSpawn" "OverrideRootScale" self null))
        (bind _asbp_weapon_base (cast `/Game/ProjEng/Core/Weapons/BP_WeaponBase` _returnvalue_2))
        (bind _output_get (set `self.CurrentWeapon` _asbp_weapon_base))
        (`self.K2_AttachToComponent` _output_get (`self.Mesh`) "Weapon" "SnapToTarget" "SnapToTarget" "KeepWorld" true)))))

(event `/Game/Blueprints/AI/BPI_Enemy.Attack`
  (params (FocusedActor :type "Actor Object Reference") (bCloseAttack :type Boolean))
  (bind _currentweapon (`self.CurrentWeapon`))
  (if bCloseAttack
    (`|PlayMontage` (`self.Mesh`) "/Game/ProjEng/Art/Characters/Worker/Animations/AM_Pistol_Whip.AM_Pistol_Whip"
      (:`then`
        (`GameplayStatics.ApplyDamage` (`GameplayStatics.GetPlayerCharacter` 0) 5.0)))
    (else
      (message `/Game/ProjEng/Data/Inventory/BPI_InventoryInteraction.Initialize` _currentweapon null)
      (`KismetSystemLibrary.RetriggerableDelay` 0.5)
      (message `/Game/ProjEng/Data/Inventory/BPI_InventoryInteraction.StopInitializing` _currentweapon))))

(event `/Game/Blueprints/Characters/BP_BaseCharacter.Death`
  (bind _currentweapon (`self.CurrentWeapon`))
  (`/Engine/EditorBlueprintResources/StandardMacros.IsValid` _currentweapon
    (:`Is Valid`
      (`/Game/ProjEng/Core/Weapons/BP_WeaponBase.DropWeapon` _currentweapon))
    (:`Is Not Valid`
      _))
  (`parent.Death`))

(fn `UserConstructionScript`
  (`parent.UserConstructionScript`))