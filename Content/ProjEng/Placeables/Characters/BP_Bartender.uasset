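; BP_Bartender is a placeable bartender character that prepares and serves a named food item.
; It caches all BP_FoodLocation actors on BeginPlay.
; MakeFood runs the latent BartenderMoves sequence: AI walk to the bottles, pick-up montage, walk to the bartending point, snap to its transform, bartending montage, completion sound.
; It then spawns BP_Food at the first cached location, passing the location and name.
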(event `self.ReceiveBeginPlay`
  (bind _outactors (`GameplayStatics.GetAllActorsOfClass` "/Game/Blueprints/WorldItems/Pub/BP_FoodLocation.BP_FoodLocation_C"))
  (set `self.FoodLocations` _outactors))

(event `MakeFood`
  (params (FoodName :type Name))
  (bind _bartendingpoint (`self.BartendingPoint`))
  (bind _output (`|GetArrayItem` (`self.FoodLocations`)))
  (`|AIMoveTo` self (0.0 0.0 0.0) (`self.CheckingBottlesPoint`) 10.0
    (:`OnSuccess`
      (`|PlayMontage` (`self.Mesh`) "/Game/ProjEng/Art/Characters/Worker/Animations/AM_Pick_Fruit.AM_Pick_Fruit"
        (:`OnBlendOut`
          (`|AIMoveTo` self (0.0 0.0 0.0) _bartendingpoint
            (:`OnSuccess`
              (`self.K2_SetActorTransform` (`self.GetTransform` _bartendingpoint))
              (`|PlayMontage` (`self.Mesh`) "/Game/ProjEng/Art/Characters/Worker/Animations/AM_Bartending.AM_Bartending"
                (:`OnCompleted`
                  (`GameplayStatics.PlaySoundAtLocation` "/Game/ProjEng/Art/Sounds/Bartender/C_BartenderComplete.C_BartenderComplete" (`self.K2_GetActorLocation`) (struct) 1.0 1.0 0.0 "/Game/ProjEng/Art/Sounds/Bartender/SA_Bartender.SA_Bartender" null null null)
                  (bind _returnvalue (`|SpawnActorFromClass` "/Game/Blueprints/WorldItems/Pub/BP_Food.BP_Food_C" (`self.GetTransform` _output) "AlwaysSpawn" "OverrideRootScale" null _output (make `/Game/ProjEng/Data/Inventory/Structures/SItem` FoodName) null))
                  (`KismetSystemLibrary.PrintString` (`KismetSystemLibrary.GetDisplayName` _returnvalue)))))))))))

(fn `UserConstructionScript`
  (`parent.UserConstructionScript`))