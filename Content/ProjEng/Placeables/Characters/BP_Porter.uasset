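; BP_Porter is an AI-controlled porter character that starts following the player in response to the hero's police spawn event.
; Shortly after BeginPlay, it casts the player character to BP_BaseHero and binds StartFollowingPlayer to the EDPoliceSpawn dispatcher.
; That handler sets CanSeePlayer to true on the AI controller's Blackboard, leaving the chase behavior to logic outside this Blueprint.
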(event `self.ReceiveBeginPlay`
  (`parent.ReceiveBeginPlay`)
  (`KismetSystemLibrary.Delay` 0.2)
  (bind _asbp_base_hero (cast `/Game/Blueprints/Characters/BP_BaseHero` (`GameplayStatics.GetPlayerCharacter` 0)))
  (add `/Game/Blueprints/Characters/BP_BaseHero.ED_PoliceSpawn` _asbp_base_hero (delegate `StartFollowingPlayer`)))

(event `StartFollowingPlayer`
  (`BlackboardComponent.SetValueAsBool` (`AIBlueprintHelperLibrary.GetBlackboard` (`AIBlueprintHelperLibrary.GetAIController` self)) "CanSeePlayer" true))

(fn `UserConstructionScript`
  (`parent.UserConstructionScript`))