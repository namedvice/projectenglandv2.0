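; BP_BaseCharacter is a base character Blueprint that provides health, damage handling and ragdoll death.
; Health starts at MaxHealth on BeginPlay, and AnyDamage subtracts incoming damage, calling Death through a DoOnce once it reaches zero or below.
; Death disables movement and capsule collision, turns on physics and collision for the mesh, and unpossesses the controller.
; Debug strings print on damage and death.
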(event `self.ReceiveBeginPlay`
  (set `self.Health` (`self.MaxHealth`)))

(event `self.ReceiveAnyDamage`
  (params (Damage :type "Float (single-precision)") (DamageType :type "DamageType Object Reference") (InstigatedBy :type "Controller Object Reference") (DamageCauser :type "Actor Object Reference"))
  (bind _output_get (set `self.Health` (- (`self.Health`) Damage)))
  (`KismetSystemLibrary.PrintString` "Damage")
  (if (<= _output_get 0.0)
    (`/Engine/EditorBlueprintResources/StandardMacros.DoOnce` false
      (:`Completed`
        (`self.Death`)))))

(event `Death`
  (bind _mesh (`self.Mesh`))
  (`CharacterMovementComponent.DisableMovement` (`self.CharacterMovement`))
  (`PrimitiveComponent.SetSimulatePhysics` _mesh true)
  (`PrimitiveComponent.SetCollisionEnabled` _mesh "QueryAndPhysics")
  (`KismetSystemLibrary.PrintString` "This Is death")
  (`PrimitiveComponent.SetCollisionEnabled` (`self.CapsuleComponent`) "NoCollision")
  (`Controller.UnPossess` (`self.GetController`)))

(fn `UserConstructionScript`)