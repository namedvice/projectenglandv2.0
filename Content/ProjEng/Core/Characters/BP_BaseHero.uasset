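; Base player hero: camera-relative movement, sprint, crouch, pause menu, and a mission-failed screen on death.
; BeginPlay loads saved currency, creates the HUD and seeds the inventory component with a pistol; input drives items and world interaction.
; Right mouse locks onto the nearest living enemy via a looping rotation timer, Tab cycles targets, and left mouse fires while aiming, otherwise punches.
; Camera-spline and journal logic remains but is disconnected.
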(event `self.ReceiveBeginPlay`
  (bind _charactermovement (`self.CharacterMovement`))
  (`parent.ReceiveBeginPlay`)
  (bind _returnvalue (`GameplayStatics.DoesSaveGameExist` "gamecurrencyinfo"))
  (if _returnvalue
    (bind _returnvalue_2 (`GameplayStatics.LoadGameFromSlot` "gamecurrencyinfo"))
    (bind _asbp_game_currency (cast `/Game/ProjEng/Core/SaveGame/BP_GameCurrency` _returnvalue_2))
    (set `self.GameCurrency` (`/Game/ProjEng/Core/SaveGame/BP_GameCurrency.GameCurrency` _asbp_game_currency))
    (else
      (set `self.GameCurrency` 250)))
  ;[1 1 1] UI Setup
  (bind _returnvalue_3 (`|CreateWidget` "/Game/ProjEng/UI/WB_UI.WB_UI_C" null self))
  (`UserWidget.AddToViewport` _returnvalue_3 0)
  (set `self.WB_UI` _returnvalue_3)
  ;[1 1 1] Inventory Updates
  (`/Game/ProjEng/Data/Inventory/Components/BP_ItemContainer.Initialize` (`self.BPC_PlayerInventory`) (`/Game/ProjEng/UI/WB_UI.WB_Inventory` (`self.WB_UI`)))
  (`/Game/ProjEng/Data/Inventory/Components/BP_ItemContainer.AddItem` (`self.BPC_PlayerInventory`) (make `/Game/ProjEng/Data/Inventory/Structures/SItem` "pistol"))
  ;[1 1 1] Set Speeds
  (set `CharacterMovementComponent.MaxWalkSpeed` (`self.WalkSpeed`) _charactermovement)
  (set `CharacterMovementComponent.MaxWalkSpeedCrouched` (`self.CrouchSpeed`) _charactermovement))

(event `Tick`
  (`AIPerceptionStimuliSourceComponent.RegisterForSense` (`self.AIPerceptionStimuliSource`) "/Script/AIModule.AISense_Sight"))

(event `GetDrunk`)

(event `InputAxis|Move Forward / Backward`
  (params (AxisValue :type "Float (single-precision)"))
  (bind (_returnvalue_x _returnvalue_y) (`KismetMathLibrary.BreakVector` (`KismetMathLibrary.GetForwardVector` (`PlayerCameraManager.GetCameraRotation` (`GameplayStatics.GetPlayerCameraManager` 0)))))
  ;[1 1 1] Moving
  (`self.AddMovementInput` (`KismetMathLibrary.MakeVector` _returnvalue_x _returnvalue_y) AxisValue))

(event `Key|V`
  (params (Key :type "Key Structure"))
  (:`Pressed`
    (`|PlayMontage` (`self.Mesh`) "/Game/ProjEng/Art/Characters/Worker/Animations/AM_Hand_Raising.AM_Hand_Raising"
      (:`then`
        (`KismetSystemLibrary.Delay` 0.5)
        (`self.ED_Cheers`)
        (`KismetSystemLibrary.PrintString` "V Pressed")))))

(event `InputAxis|Move Right / Left`
  (params (AxisValue :type "Float (single-precision)"))
  (bind (_returnvalue_x _returnvalue_y) (`KismetMathLibrary.BreakVector` (`KismetMathLibrary.GetRightVector` (`PlayerCameraManager.GetCameraRotation` (`GameplayStatics.GetPlayerCameraManager` 0)))))
  ;[1 1 1] Moving
  (`self.AddMovementInput` (`KismetMathLibrary.MakeVector` _returnvalue_x _returnvalue_y) AxisValue))

(event `Key|C`
  (params (Key :type "Key Structure"))
  ;[1 1 1] Moving
  (:`Pressed`
    (`/Engine/EditorBlueprintResources/StandardMacros.FlipFlop`
      (:`A`
        (`self.Crouch`))
      (:`B`
        (`self.UnCrouch`)))))

(event `self.ReceiveTick`
  (params (DeltaSeconds :type "Float (single-precision)")))

(event `EveryoneStartSprint`
  ;[1 1 1] Sprint
)

(event `StartSprint`
  ;[1 1 1] Sprint
  (`self.EveryoneStartSprint`))

(event `StopSprint`
  ;[1 1 1] Sprint
  (`self.EveryoneStopSprint`))

(event `EveryoneStopSprint`
  ;[1 1 1] Sprint
)

(event `Key|J`
  (params (Key :type "Key Structure"))
  ;[1 1 1] Journal Interaction
)

(event `InputAction|Sprint`
  (params (Key :type "Key Structure"))
  (bind _charactermovement (`self.CharacterMovement`))
  ;[1 1 1] Sprint
  (:`Pressed`
    (set `CharacterMovementComponent.MaxWalkSpeed` (`self.SprintSpeed`) _charactermovement)
    (set `CharacterMovementComponent.MaxWalkSpeedCrouched` (`self.CrouchSprintSpeed`) _charactermovement))
  (:`Released`
    (set `CharacterMovementComponent.MaxWalkSpeed` (`self.WalkSpeed`) _charactermovement)
    (set `CharacterMovementComponent.MaxWalkSpeedCrouched` (`self.CrouchSpeed`) _charactermovement)))

(event `Key|Escape`
  (params (Key :type "Key Structure"))
  ;[1 1 1] In Game Options
  (:`Pressed`
    (if (not (`PlayerController.bShowMouseCursor` (`GameplayStatics.GetPlayerController` 0)))
      (bind _returnvalue (`|CreateWidget` "/Game/ProjEng/Maps/WB_InGameMenu.WB_InGameMenu_C"))
      (`UserWidget.AddToViewport` _returnvalue 0)
      (`self.DisableInput` (`GameplayStatics.GetPlayerController` 0))
      (`GameplayStatics.SetGamePaused` true))))

(event `Key|L`
  (params (Key :type "Key Structure"))
  ;[1 1 1] Inventory
  ;;[1 1 1] Inventory Debug
  (:`Pressed`
    (`KismetSystemLibrary.PrintString` (`KismetStringLibrary.Conv_IntToString` (`KismetArrayLibrary.Array_Length` (`/Game/ProjEng/Data/Inventory/Components/BPC_PlayerInventory.NearbyItems` (`self.BPC_PlayerInventory`)))))))

(event `Key|G`
  (params (Key :type "Key Structure"))
  ;[1 1 1] Inventory
  (:`Pressed`
    (`/Game/ProjEng/Data/Inventory/Components/BPC_PlayerInventory.DropItemFromHands` (`self.BPC_PlayerInventory`))))

(event `Key|One`
  (params (Key :type "Key Structure"))
  ;[1 1 1] Inventory
  ;;[1 1 1] Slots Switch
  (:`Pressed`
    (`/Game/ProjEng/UI/Inventory/WB_Inventory.ChangeActiveSlot` (`/Game/ProjEng/Data/Inventory/Components/BP_ItemContainer.WB_Inventory` (`self.BPC_PlayerInventory`)) 0)))

(event `Key|Two`
  (params (Key :type "Key Structure"))
  ;[1 1 1] Inventory
  ;;[1 1 1] Slots Switch
  (:`Pressed`
    (`/Game/ProjEng/UI/Inventory/WB_Inventory.ChangeActiveSlot` (`/Game/ProjEng/Data/Inventory/Components/BP_ItemContainer.WB_Inventory` (`self.BPC_PlayerInventory`)) 1)))

(event `Key|Three`
  (params (Key :type "Key Structure"))
  ;[1 1 1] Inventory
  ;;[1 1 1] Slots Switch
  (:`Pressed`
    (`/Game/ProjEng/UI/Inventory/WB_Inventory.ChangeActiveSlot` (`/Game/ProjEng/Data/Inventory/Components/BP_ItemContainer.WB_Inventory` (`self.BPC_PlayerInventory`)) 2)))

(event `Key|F`
  (params (Key :type "Key Structure"))
  ;[1 1 1] Inventory
  (:`Pressed`
    (bind _success (`/Game/ProjEng/Data/Inventory/Components/BPC_PlayerInventory.UseItem` (`self.BPC_PlayerInventory`)))
    (if _success
      _)))

(event `Key|LeftMouseButton`
  (params (Key :type "Key Structure"))
  ;[1 1 1] Inventory
  ;;[1 1 1] Weapon Attack
  (:`Pressed`
    (if (`self.bAiming`)
      (bind _currentweapon (`self.CurrentWeapon`)
        (:`then`
          (`/Game/ProjEng/Core/Weapons/BP_WeaponBase.Initialize` _currentweapon null))
        (:`else`
          (`self.Attack` :!label _label)))
      (else
        (goto _label))))
  (:`Released`
    (bind _currentweapon_2 (`self.CurrentWeapon`)
      (:`then`
        (`/Game/ProjEng/Core/Weapons/BP_WeaponBase.StopInitializing` _currentweapon_2))
      (:`else`))))

(event `InputAction|Interact`
  (params (Key :type "Key Structure"))
  (bind _bpc_worldinteraction (`self.BPC_WorldInteraction`))
  ;[1 1 1] Inventory
  (:`Pressed`
    (`/Engine/EditorBlueprintResources/StandardMacros.IsValid` (`/Game/ProjEng/Core/Engine/Components/WorldInteraction/BP_WorldInteraction.NearWorldItem` _bpc_worldinteraction)
      (:`Is Valid`
        (`/Game/ProjEng/Core/Engine/Components/WorldInteraction/BP_WorldInteraction.InteractWithWorldItem` _bpc_worldinteraction))
      (:`Is Not Valid`
        (`/Engine/EditorBlueprintResources/StandardMacros.IsValid` (`|GetArrayItem` (`/Game/ProjEng/Data/Inventory/Components/BPC_PlayerInventory.NearbyItems` (`self.BPC_PlayerInventory`)))
          (:`Is Valid`
            (`/Game/ProjEng/Data/Inventory/Components/BPC_PlayerInventory.Interact` (`self.BPC_PlayerInventory`)))))))
  (:`Released`
    (`/Game/ProjEng/Core/Engine/Components/WorldInteraction/BP_WorldInteraction.StopInteracting` _bpc_worldinteraction)))

(event `Key|RightMouseButton`
  (params (Key :type "Key Structure"))
  ;[1 1 1] Focusing Enemy
  (:`Pressed`
    (`/Engine/EditorBlueprintResources/StandardMacros.IsValid` (`self.CurrentWeapon`)
      (:`Is Valid`
        (bind (_closestenemyactor _success) (`self.GetClosestEnemy` (`PrimitiveComponent.GetOverlappingActors` (`self.EnemiesSense`) "/Game/ProjEng/Core/Characters/BP_BaseEnemy.BP_BaseEnemy_C")))
        (if _success
          (set `self.ClosestEnemy` _closestenemyactor)
          (set `self.bAiming` true)
          (bind _returnvalue (`KismetSystemLibrary.K2_SetTimerDelegate` (delegate `RotateToClosestEnemy`) 0.005 true))
          (set `self.RotateToEnemyTimer` _returnvalue)))))
  (:`Released`
    (`KismetSystemLibrary.K2_ClearAndInvalidateTimerHandle` (`self.RotateToEnemyTimer`) :!label _label_2)
    (set `self.bAiming` false)
    (bind _currentweapon (`self.CurrentWeapon`)
      (:`then`
        (`/Game/ProjEng/Core/Weapons/BP_WeaponBase.StopInitializing` _currentweapon))
      (:`else`))))

(event `StopAiming`
  ;[1 1 1] Focusing Enemy
  (goto _label_2))

(event `RotateToClosestEnemy`
  (bind _closestenemy (`self.ClosestEnemy`))
  (bind _closestenemy_2 (`self.ClosestEnemy`))
  ;[1 1 1] Focusing Enemy
  (`/Engine/EditorBlueprintResources/StandardMacros.IsValid` _closestenemy_2
    (:`Is Valid`
      (`/Game/ProjEng/Core/Characters/BP_BaseEnemy.Highlight` _closestenemy_2)
      (`SceneComponent.K2_SetWorldRotation` (`self.CapsuleComponent`) (`KismetMathLibrary.MakeRotator` 0.0 0.0 (.yaw (`KismetMathLibrary.FindLookAtRotation` (`self.K2_GetActorLocation`) (`self.K2_GetActorLocation` _closestenemy_2)))) false false)
      (if (<= (`self.GetDistanceTo` _closestenemy) (`SphereComponent.SphereRadius` (`self.EnemiesSense`)))
        (if (`/Game/ProjEng/Core/Characters/BP_BaseEnemy.Dead` _closestenemy)
          (`self.ChangeActorInFocus` (`PrimitiveComponent.GetOverlappingActors` (`self.EnemiesSense`) "/Game/ProjEng/Core/Characters/BP_BaseEnemy.BP_BaseEnemy_C")))))))

(event `Key|Tab`
  (params (Key :type "Key Structure"))
  ;[1 1 1] Focusing Enemy
  (:`Pressed`
    (`self.ChangeActorInFocus` (`PrimitiveComponent.GetOverlappingActors` (`self.EnemiesSense`) "/Game/ProjEng/Core/Characters/BP_BaseEnemy.BP_BaseEnemy_C"))))

(event `Key|R`
  (params (Key :type "Key Structure"))
  ;[1 1 1] Focusing Enemy
  (:`Pressed`
    (bind _currentweapon (`self.CurrentWeapon`)
      (:`then`
        (`/Game/ProjEng/Core/Weapons/BP_WeaponBase.Reload` _currentweapon))
      (:`else`))))

(event `Attack`
  ;[1 1 1] Attack
  (if (not (`self.bAttacking`))
    (set `self.bAttacking` true)
    (`|PlayMontage` (`self.Mesh`) "/Game/ProjEng/Art/Characters/Worker/Animations/AM_Punching.AM_Punching"
      (:`then`
        (`KismetSystemLibrary.Delay` 0.2)
        (for _array_element (`PrimitiveComponent.GetOverlappingActors` (`self.AttackBox`) "/Script/Engine.Actor")
          (`GameplayStatics.ApplyDamage` _array_element 30.0))
        (`GameplayStatics.PlaySound2D` "/Game/ProjEng/Art/Sounds/Footsteps/A_HeavyWoodFootstep2.A_HeavyWoodFootstep2" 1.0 1.0 0.0 null null))
      (:`OnCompleted`
        (set `self.bAttacking` false)))))

(event `self.Death`
  (message `/Game/ProjEng/Data/Inventory/BPI_InventoryInteraction.StopInitializing` (`self.CurrentWeapon`))
  (`parent.Death`)
  (`KismetSystemLibrary.Delay` 1.0)
  (bind _returnvalue (`|CreateWidget` "/Game/ProjEng/UI/MissionResult/WB_MissionResult.WB_MissionResult_C"))
  (`UserWidget.AddToViewport` _returnvalue 0))

(fn `ChangeActorInFocus`
  (params (TargetArray :type "Array of Actor Object Reference (by ref)"))
  (if (== (`KismetArrayLibrary.Array_Length` TargetArray) 0)
    (set `self.ClosestEnemy` null)
    (set `self.CurrentActorInFocusIndex` 0)
    (`self.StopAiming`)
    (else
      (bind _output_get (set `self.CurrentActorInFocusIndex` (+ (`self.CurrentActorInFocusIndex`) 1)))
      (if (>= _output_get (`KismetArrayLibrary.Array_Length` TargetArray))
        (set `self.CurrentActorInFocusIndex` 0))
      (bind _asbp_base_enemy (cast `/Game/ProjEng/Core/Characters/BP_BaseEnemy` (`|GetArrayItem` TargetArray (`self.CurrentActorInFocusIndex`))))
      (set `self.ClosestEnemy` _asbp_base_enemy)))
  (return))

(fn `GetClosestEnemy`
  (params (Array :type "Array of Actor Object Reference"))
  (returns (ClosestEnemyActor :type "/Game/ProjEng/Core/Characters/BP_BaseEnemy Object Reference") (Success :type Boolean))
  (locals (LClosestEnemy :type "/Game/ProjEng/Core/Characters/BP_BaseEnemy Object Reference") (LClosestDistance :type "Float (double-precision)"))
  (bind _lclosestenemy (`local.LClosestEnemy`))
  (bind _lclosestenemy_2 (`local.LClosestEnemy`))
  (bind _returnvalue (`self.GetDistanceTo` _lclosestenemy))
  (set `local.LClosestEnemy` null)
  (for _array_element Array
    (bind _asbp_base_enemy (cast `/Game/ProjEng/Core/Characters/BP_BaseEnemy` _array_element))
    (if (not (`/Game/ProjEng/Core/Characters/BP_BaseEnemy.Dead` _asbp_base_enemy))
      (`/Engine/EditorBlueprintResources/StandardMacros.IsValid` _lclosestenemy
        (:`Is Valid`
          (if (< _returnvalue (`local.LClosestDistance`))
            (set `local.LClosestDistance` _returnvalue :!label _label)
            (set `local.LClosestEnemy` _asbp_base_enemy)))
        (:`Is Not Valid`
          (goto _label)))))
  (return _lclosestenemy_2 (`KismetSystemLibrary.IsValid` _lclosestenemy_2)))

(fn `UserConstructionScript`
  (`parent.UserConstructionScript`))