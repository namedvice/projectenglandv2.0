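; BP_WorldItem is an interactable world item that can be used, or dropped from the player's hands.
; Box or sphere overlap registers it with the visitor's BP_WorldInteraction and scales its prompt widget in or out.
; OnInteract calls the empty PostInteraction hook immediately or after a progress timeline, which StopInitializing can halt.
; OnDrop detaches it, re-enables interaction, launches it along the player's forward vector and clears the inventory's held item.
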(event `self.ReceiveBeginPlay`
  ;[1 1 1] BeginPlay
  (if (`self.bInteractionDisabledByDefault`)
    (`self.DisableInteraction`))
  (`PrimitiveComponent.SetCollisionEnabled` (select `bool` (`self.bSphereCollision`) :`false` (`self.Sphere`) :`true` (`self.Box`) :!type "PrimitiveComponent Object Reference") "NoCollision")
  (`PrimitiveComponent.SetCollisionEnabled` (select `bool` (`self.bSphereCollision`) :`false` (`self.Box`) :`true` (`self.Sphere`) :!type "PrimitiveComponent Object Reference") "QueryAndPhysics")
  (bind _aswb_interact_button (cast `/Game/UI/InteractionWidgets/WB_InteractButton` (`WidgetComponent.GetUserWidgetObject` (`self.WidgetInteraction`))))
  (bind _output_get (set `self.InteractWidget` _aswb_interact_button))
  (`/Game/UI/InteractionWidgets/WB_InteractButton.SetDotColor` _output_get (`self.WidgetDotType`)))

(event `self.ReceiveTick`
  (params (DeltaSeconds :type "Float (single-precision)")))

(event `DisableInteraction`
  ;[1 1 1] Initialization
  (set `PrimitiveComponent.bGenerateOverlapEvents` false (`self.Sphere`))
  (set `PrimitiveComponent.bGenerateOverlapEvents` false (`self.Box`))
  (`SceneComponent.SetVisibility` (`self.InteractionWidg`) false true))

(event `/Game/ProjEng/Data/Inventory/BPI_InventoryInteraction.OnInteract`
  (params (Actor :type "Actor Object Reference"))
  ;[1 1 1] Initialization
  (switch `/Game/ProjEng/Data/EInteractionType` (`self.InteractionType`)
    (:`NewEnumerator2`
      (`self.PostInteraction` :!label _label))
    (:`NewEnumerator0`
      (bind _direction (`Timeline|Timeline_0` :!via `PlayFromStart` :!label _label_2)
        (:`Finished`
          (if (`|EnumEquality` _direction "Forward")
            (`KismetSystemLibrary.PrintString` "InteractionEnded" true true (struct :`R` 1.0 :`G` 0.096244 :`B` 0.50083 :`A` 1.0))
            (goto _label)))))))

(event `/Game/ProjEng/Data/Inventory/BPI_InventoryInteraction.StopInitializing`
  ;[1 1 1] Initialization
  (goto _label_2 :!via `Stop`))

(event `EnableInteraction`
  ;[1 1 1] Initialization
  (set `PrimitiveComponent.bGenerateOverlapEvents` true (`self.Box`))
  (set `PrimitiveComponent.bGenerateOverlapEvents` true (`self.Sphere`))
  (`SceneComponent.SetVisibility` (`self.InteractionWidg`) true true))

(event `PostInteraction`
  ;[1 1 1] Initialization
)

(event `/Game/ProjEng/Data/Inventory/BPI_InventoryInteraction.OnDrop`
  (bind _returnvalue (`self.GetComponentByClass` (`GameplayStatics.GetPlayerCharacter` 0) "/Game/ProjEng/Data/Inventory/Components/BPC_PlayerInventory.BPC_PlayerInventory_C"))
  ;[1 1 1] Drop
  (`self.K2_DetachFromActor` "KeepWorld" "KeepWorld" "KeepWorld")
  (`self.EnableInteraction`)
  (`self.SetOwner` null)
  (`PrimitiveComponent.SetSimulatePhysics` (`self.StaticMesh`) true)
  (`PrimitiveComponent.SetAllPhysicsLinearVelocity` (`self.StaticMesh`) (0.0 0.0 0.0) false)
  (`PrimitiveComponent.AddImpulse` (`self.StaticMesh`) (* (`self.GetActorForwardVector` (`GameplayStatics.GetPlayerCharacter` 0)) 500.0) "None" true)
  (set `/Game/ProjEng/Data/Inventory/Components/BPC_PlayerInventory.bHoldingSomething` false _returnvalue)
  (set `/Game/ProjEng/Data/Inventory/Components/BPC_PlayerInventory.HandsItem` null _returnvalue))

(event `self.Box.OnComponentBeginOverlap`
  (params (OverlappedComponent :type "PrimitiveComponent Object Reference") (OtherActor :type "Actor Object Reference") (OtherComp :type "PrimitiveComponent Object Reference") (OtherBodyIndex :type Integer) (bFromSweep :type Boolean) (SweepResult :type "HitResult Structure (by ref)"))
  (bind _interactwidget (`self.InteractWidget`))
  ;[1 1 1] Overlap
  (bind _returnvalue (`self.GetComponentByClass` (select `bool` (`self.bSphereCollision`) :`false` OtherActor :`true` (stale `self.Sphere.OnComponentBeginOverlap` OtherActor)) "/Game/ProjEng/Core/Engine/Components/WorldInteraction/BP_WorldInteraction.BP_WorldInteraction_C"))
  (`/Engine/EditorBlueprintResources/StandardMacros.IsValid` _returnvalue :!label _label_3
    (:`Is Valid`
      (set `/Game/ProjEng/Core/Engine/Components/WorldInteraction/BP_WorldInteraction.NearWorldItem` self _returnvalue)
      (`/Engine/EditorBlueprintResources/StandardMacros.IsValid` _interactwidget
        (:`Is Valid`
          (bind (_direction _scale) (`Timeline|Timeline_1` :!label _label_4)
            (:`Update`
              (`SceneComponent.SetWorldScale3D` (`self.InteractionWidg`) (`KismetMathLibrary.Conv_DoubleToVector` _scale)))
            (:`Finished`
              (switch `ETimelineDirection` _direction
                (:`Forward`
                  (`/Game/UI/InteractionWidgets/WB_InteractButton.ShowHide` _interactwidget true))))))))))

(event `self.Sphere.OnComponentBeginOverlap`
  (params (OverlappedComponent :type "PrimitiveComponent Object Reference") (OtherActor :type "Actor Object Reference") (OtherComp :type "PrimitiveComponent Object Reference") (OtherBodyIndex :type Integer) (bFromSweep :type Boolean) (SweepResult :type "HitResult Structure (by ref)"))
  ;[1 1 1] Overlap
  (goto _label_3))

(event `self.Box.OnComponentEndOverlap`
  (params (OverlappedComponent :type "PrimitiveComponent Object Reference") (OtherActor :type "Actor Object Reference") (OtherComp :type "PrimitiveComponent Object Reference") (OtherBodyIndex :type Integer))
  (bind _interactwidget (`self.InteractWidget`))
  ;[1 1 1] Overlap
  (bind _returnvalue (`self.GetComponentByClass` (select `bool` (`self.bSphereCollision`) :`false` OtherActor :`true` (stale `self.Sphere.OnComponentEndOverlap` OtherActor)) "/Game/ProjEng/Core/Engine/Components/WorldInteraction/BP_WorldInteraction.BP_WorldInteraction_C"))
  (`/Engine/EditorBlueprintResources/StandardMacros.IsValid` _returnvalue :!label _label_5
    (:`Is Valid`
      (set `/Game/ProjEng/Core/Engine/Components/WorldInteraction/BP_WorldInteraction.NearWorldItem` null _returnvalue)
      (`/Engine/EditorBlueprintResources/StandardMacros.IsValid` _interactwidget
        (:`Is Valid`
          (`KismetSystemLibrary.RetriggerableDelay` 0.2)
          (`/Game/UI/InteractionWidgets/WB_InteractButton.ShowHide` _interactwidget false)
          (goto _label_4 :!via `Reverse`))))))

(event `self.Sphere.OnComponentEndOverlap`
  (params (OverlappedComponent :type "PrimitiveComponent Object Reference") (OtherActor :type "Actor Object Reference") (OtherComp :type "PrimitiveComponent Object Reference") (OtherBodyIndex :type Integer))
  ;[1 1 1] Overlap
  (goto _label_5))

(fn `UserConstructionScript`)