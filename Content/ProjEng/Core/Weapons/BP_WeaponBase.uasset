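; Base weapon Blueprint that the hero picks up, fires, reloads and drops, and that also fires for enemy owners.
; Stats load from DT_Weapons by ID; interacting attaches it to the hero's weapon socket.
; A looping timer fires hero bullets at ClosestEnemy or enemy bullets at the player, based on owner.
; Only hero shots use ammo; an empty clip triggers a montage-timed reload, or a physics drop without reserves.
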(event `AddAmmo`
  (params (Amount :type Integer))
  (set `self.ClipseAmmo` (+ (`self.ClipseAmmo`) Amount)))

(event `self.ReceiveBeginPlay`
  ;[1 1 1] Begin Play
  (`PrimitiveComponent.SetCollisionEnabled` (`self.Sphere`) "NoCollision")
  (`KismetSystemLibrary.PrintString` "ThereGoes The Weapon!")
  (bind _returnvalue (`|GetDataTableRow` "/Game/ProjEng/Core/Weapons/DT_Weapons.DT_Weapons" (`self.ID`))
    (:`then`
      (bind _output_get (set `self.Info` _returnvalue))
      (set `self.CurrentAmmo` (`.MaxClipseAmmo_15_E8CFD41A4976C8B06E4530A0D83A7056` (break `/Game/ProjEng/Core/Weapons/SWeaponInfo` _output_get))))))

(event `self.OnInteract`
  (params (Actor :type "Actor Object Reference"))
  (bind _character (`self.Character`))
  ;[1 1 1] Take Weapon
  (`/Engine/EditorBlueprintResources/StandardMacros.IsValid` (`self.Character`)
    (:`Is Valid`
      _)
    (:`Is Not Valid`
      (bind _asbp_base_hero (cast `/Game/Blueprints/Characters/BP_BaseHero` (`GameplayStatics.GetPlayerCharacter` 0)))
      (set `self.Character` _asbp_base_hero)))
  (bind _currentweapon (`/Game/Blueprints/Characters/BP_BaseHero.CurrentWeapon` (`self.Character`))
    (:`then`
      (`self.DropWeapon` _currentweapon))
    (:`else`
      _))
  (`PrimitiveComponent.SetSimulatePhysics` (`self.StaticMesh`) false)
  (`self.K2_AttachToComponent` (`Character.Mesh` _character) (`SkinnedMeshComponent.GetSocketBoneName` (`Character.Mesh` _character) "weapon") "SnapToTarget" "SnapToTarget" "SnapToTarget")
  (set `/Game/Blueprints/Characters/BP_BaseHero.CurrentWeapon` self _character)
  (`self.SetOwner` (`self.Character`))
  (`PrimitiveComponent.SetCollisionEnabled` (`self.Sphere`) "NoCollision")
  (`PrimitiveComponent.SetCollisionEnabled` (`self.StaticMesh`) "NoCollision"))

(event `DropWeapon`
  ;[1 1 1] Drop Weapon
  (`self.StopInitializing`)
  (`self.K2_DetachFromActor` "KeepWorld" "KeepWorld" "KeepWorld")
  (`PrimitiveComponent.SetCollisionEnabled` (`self.StaticMesh`) "QueryAndPhysics")
  (`PrimitiveComponent.SetCollisionEnabled` (`self.Sphere`) "QueryAndPhysics")
  (`PrimitiveComponent.SetSimulatePhysics` (`self.StaticMesh`) true)
  (`PrimitiveComponent.AddImpulse` (`self.StaticMesh`) (* (`self.GetActorForwardVector` (`self.GetOwner`)) 200.0) "None" true)
  (bind _asbp_base_hero (cast `/Game/Blueprints/Characters/BP_BaseHero` (`self.GetOwner`)))
  (`/Game/Blueprints/Characters/BP_BaseHero.StopAiming` _asbp_base_hero))

(event `self.Initialize`
  (params (Initializator :type "Actor Object Reference"))
  (bind ((`FireRate_5_EEC4FA104582F6442DFA9FB167130458` _firerate)) (break `/Game/ProjEng/Core/Weapons/SWeaponInfo` (`self.Info`)))
  ;[1 1 1] Initialize
  (`/Engine/EditorBlueprintResources/StandardMacros.DoOnce` false :!label _label
    (:`Completed`
      (`self.Fire`)
      (bind _returnvalue (`KismetSystemLibrary.K2_SetTimerDelegate` (delegate `Fire`) _firerate true))
      (set `self.FireTimer` _returnvalue)
      (`KismetSystemLibrary.Delay` _firerate)
      (goto _label :!via `Reset`))))

(event `Fire`
  (bind _returnvalue (`self.GetOwner`))
  (bind _returnvalue_2 (`self.GetOwner`))
  (bind _returnvalue_3 (`GameplayStatics.GetPlayerCharacter` 0))
  (bind ((`Damage_7_35C177804C89395C5F932FA7465E6B8A` _damage)) (break `/Game/ProjEng/Core/Weapons/SWeaponInfo` (`self.Info`)))
  (bind _returnvalue_location (`KismetMathLibrary.BreakTransform` (`SceneComponent.GetSocketTransform` (`self.StaticMesh`) "muzzle" "RTS_World")))
  (bind _returnvalue_4 (`self.K2_GetActorLocation` _returnvalue_3))
  (bind _closestenemy (`/Game/Blueprints/Characters/BP_BaseHero.ClosestEnemy` (`self.Character`)))
  ;[1 1 1] Initialize
  (if (not (`self.bReloading`))
    (`GameplayStatics.SpawnSoundAtLocation` "/Game/Sounds/Gunshots/C_Gunshots.C_Gunshots" (`self.K2_GetActorLocation` (`self.GetOwner`)) (struct) 1.0 1.0 0.0 null null)
    (`/Engine/EditorBlueprintResources/StandardMacros.IsValid` _returnvalue_3
      (:`Is Valid`
        (if (== _returnvalue _returnvalue_3)
          ;[1 1 1] Bullets+muzzle
          (`/Engine/EditorBlueprintResources/StandardMacros.IsValid` _closestenemy
            (:`Is Valid`
              (`|SpawnActorFromClass` "/Game/ProjEng/Core/Weapons/BP_HeroBullet.BP_HeroBullet_C" (`KismetMathLibrary.MakeTransform` _returnvalue_location (`KismetMathLibrary.FindLookAtRotation` _returnvalue_4 (`self.K2_GetActorLocation` _closestenemy)) (0.8 0.8 0.8)) "AlwaysSpawn" "OverrideRootScale" _returnvalue_2 _damage null)
              ;[1 1 1] Check for reload and Drop
              (`/Engine/EditorBlueprintResources/StandardMacros.DecrementInt` (`self.CurrentAmmo`)
                (:`  `
                  (if (> (`self.CurrentAmmo`) 0)
                    _
                    (elif (> (`self.ClipseAmmo`) 0)
                      (`self.Reload`)
                      (else
                        (`self.DropWeapon`)
                        (`self.StopInitializing`)
                        (set `/Game/Blueprints/Characters/BP_BaseHero.CurrentWeapon` null (`self.Character`))
                        (`PrimitiveComponent.SetCollisionEnabled` (`self.Sphere`) "NoCollision"))))))))
          (else
            (`|SpawnActorFromClass` "/Game/ProjEng/Core/Weapons/BP_EnemyBullet.BP_EnemyBullet_C" (`KismetMathLibrary.MakeTransform` _returnvalue_location (`KismetMathLibrary.FindLookAtRotation` (`self.K2_GetActorLocation` _returnvalue) _returnvalue_4) (0.8 0.8 0.8)) "AlwaysSpawn" "OverrideRootScale" _returnvalue_2 _damage null)))))))

(event `self.StopInitializing`
  ;[1 1 1] Initialize
  (`KismetSystemLibrary.K2_ClearAndInvalidateTimerHandle` (`self.FireTimer`)))

(event `Reload`
  (bind _clipseammo (`self.ClipseAmmo`))
  (bind ((`MaxClipseAmmo_15_E8CFD41A4976C8B06E4530A0D83A7056` _maxclipseammo)) (break `/Game/ProjEng/Core/Weapons/SWeaponInfo` (`self.Info`)))
  ;[1 1 1] Reload
  (`GameplayStatics.PlaySound2D` "/Game/Sounds/Interactions/A_Reload.A_Reload" 1.0 1.0 0.0 null null)
  (if (< (`self.CurrentAmmo`) (`.MaxClipseAmmo_15_E8CFD41A4976C8B06E4530A0D83A7056` (break `/Game/ProjEng/Core/Weapons/SWeaponInfo` (`self.Info`))))
    (set `self.bReloading` true)
    (`|PlayMontage` (`Character.Mesh` (`GameplayStatics.GetPlayerCharacter` 0)) "/Game/ProjEng/Art/Characters/Worker/Animations/AM_Reloading.AM_Reloading"
      (:`OnCompleted`
        (if (>= _clipseammo _maxclipseammo)
          (set `self.CurrentAmmo` _maxclipseammo)
          (set `self.ClipseAmmo` (- _clipseammo (- _maxclipseammo (`self.CurrentAmmo`))))
          (else
            (set `self.CurrentAmmo` (`self.ClipseAmmo`))
            (set `self.ClipseAmmo` 0)))
        (set `self.bReloading` false)))))

(fn `UserConstructionScript`)