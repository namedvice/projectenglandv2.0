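; BP_EnemyBullet is an enemy projectile that damages what it hits by chance and lives at most one second.
; On spawn, it samples a curve with the distance between its owner and the player to set its hit chance.
; A sphere hit on an actor other than the owner rolls that chance and applies a third of Damage on success.
; Any hit destroys the bullet.
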(event `self.ReceiveBeginPlay`
  (set `self.HitChance` (`CurveFloat.GetFloatValue` (`self.HitChanceCurve`) (`self.GetDistanceTo` (`self.GetOwner`) (`GameplayStatics.GetPlayerCharacter` 0))))
  (`KismetSystemLibrary.Delay` 1.0)
  (`self.K2_DestroyActor` :!label _label))

(event `self.Sphere.OnComponentHit`
  (params (HitComponent :type "PrimitiveComponent Object Reference") (OtherActor :type "Actor Object Reference") (OtherComp :type "PrimitiveComponent Object Reference") (NormalImpulse :type "Vector Structure") (Hit :type "HitResult Structure (by ref)"))
  (bind _returnvalue (`self.GetOwner`))
  (if (and (!= OtherActor _returnvalue) (`KismetMathLibrary.InRange_FloatFloat` (`KismetMathLibrary.RandomFloatInRange` 0.0 1.0) 0.0 (`self.HitChance`)))
    (`GameplayStatics.ApplyDamage` OtherActor (/ (`self.Damage`) 3.0) null _returnvalue)
    (goto _label)
    (else
      (goto _label))))

(fn `UserConstructionScript`)