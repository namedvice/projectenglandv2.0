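; GM_House is the house game mode, which spawns and possesses the BP_BaseHero on BeginPlay.
; LoadLevel swaps streamed levels behind a camera fade using fixed delays, moves the player to a PlayerStart, retargets the camera and removes the level transition after Shop.
; Police notifier, clock-driven boat spawning, contraband addresses and crate randomisation remain, but their setup chains are disconnected.
; SetContraband and UpdateNPCs are empty stubs.
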(event `self.ReceiveBeginPlay`
  (bind _returnvalue (`|SpawnActorFromClass` "/Game/Blueprints/Characters/BP_BaseHero.BP_BaseHero_C" (`KismetMathLibrary.MakeTransform` (0.0 0.0 1000.0)) "AlwaysSpawn" "OverrideRootScale" null null null))
  (`Controller.Possess` (`GameplayStatics.GetPlayerController` 0) _returnvalue))

(event `CallReinforcement`
  (bind _notifierwidget (`self.NotifierWidget`))
  (`/Game/ProjEng/UI/Notifiers/WB_Notifier.NewNotifier` _notifierwidget "Police")
  (`/Game/ProjEng/UI/Notifiers/WB_Notifier.StartTruckArrival timer` _notifierwidget))

(event `LoadLevel`
  (params (LevelName :type Name) (CurrentLevelName :type Name))
  ;[1 1 1] Load Level
  (`self.DisableInput` (`GameplayStatics.GetPlayerCharacter` 0) (`GameplayStatics.GetPlayerController` 0))
  (`PlayerCameraManager.StartCameraFade` :`self` (`GameplayStatics.GetPlayerCameraManager` 0) :`ToAlpha` 1.0 :`Duration` 1.0 :`bHoldWhenFinished` true)
  (`KismetSystemLibrary.Delay` 1.0)
  (`CharacterMovementComponent.SetMovementMode` (`Character.CharacterMovement` (`GameplayStatics.GetPlayerCharacter` 0)) "MOVE_None" 0)
  (bind _output_get (set `self.PreviousLevelName` CurrentLevelName))
  (`GameplayStatics.UnloadStreamLevel` _output_get)
  (`GameplayStatics.LoadStreamLevel` LevelName true)
  (`CharacterMovementComponent.SetMovementMode` (`Character.CharacterMovement` (`GameplayStatics.GetPlayerCharacter` 0)) "MOVE_Walking" 0)
  (`KismetSystemLibrary.Delay` 1.0)
  (`PlayerCameraManager.StartCameraFade` :`self` (`GameplayStatics.GetPlayerCameraManager` 0) :`FromAlpha` 1.0 :`Duration` 1.0)
  (bind _returnvalue (`GameplayStatics.GetActorOfClass` "/Script/Engine.PlayerStart"))
  (`self.K2_SetActorTransform` (`GameplayStatics.GetPlayerCharacter` 0) (`self.GetTransform` _returnvalue) false false)
  (`self.EnableInput` (`GameplayStatics.GetPlayerCharacter` 0) (`GameplayStatics.GetPlayerController` 0))
  (bind _outactors (`GameplayStatics.GetAllActorsOfClass` "/Script/Engine.CameraActor"))
  (bind _output (`|GetArrayItem` _outactors 1))
  (`PlayerController.SetViewTargetWithBlend` (`GameplayStatics.GetPlayerController` 0) _output 0.0 "VTBlend_Linear" 0.0 false)
  ;[0.9016 1 0] Specify the Store level Name!!!
  (`KismetSystemLibrary.PrintString` (`KismetSystemLibrary.GetDisplayName` _output))
  (if (== (`self.PreviousLevelName`) "Shop")
    (bind _returnvalue_2 (`GameplayStatics.GetActorOfClass` "/Game/Blueprints/WorldItems/LevelsTransition/BP_LevelTransition.BP_LevelTransition_C"))
    (`self.K2_DestroyActor` _returnvalue_2)))

(event `LossGM`
  ;[0.2552 0.09139 0] Old
  (for (_array_element _array_index) (`self.PlayersControllers`)
    (`self.DisableInput` (`GameplayStatics.GetPlayerCharacter` _array_index) _array_element)))

(event `StartTimeTimer`
  (`KismetSystemLibrary.K2_SetTimerDelegate` (delegate `IncreaseTime`) 1.0 true))

(event `IncreaseTime`
  (bind _sresources (`self.SResources`))
  (bind (_hours _minutes) (break `Timecode` (`self.CurrentTime`)))
  (bind (_hours_2 _minutes_2) (break `Timecode` (`self.CurrentTime`)))
  (bind _output (`|GetArrayItem` _sresources))
  (bind _returnvalue (+ _minutes 1))
  (if (>= _returnvalue 60)
    (set `self.CurrentTime` (make `Timecode` (+ _hours 1)))
    (else
      (set `self.CurrentTime` (make `Timecode` _hours _returnvalue))))
  ;[1 1 1] Check if the Time Has Come!
  (for _array_element (`self.BoatsTime`)
    (bind (_hours_3 _minutes_3) (break `Timecode` _array_element))
    (if (and (== _hours_3 _hours_2) (== _minutes_3 _minutes_2))
      (`/Game/ProjEng/Art/House/Boat/BP_BoatSpawner.SpawnBoat` (`self.BoatSpawner`) _output)
      (`KismetArrayLibrary.Array_RemoveItem` _sresources _output)
      (break)))
  (`self.UpdateNPCs`))

(event `self.K2_PostLogin`
  (params (NewPlayer :type "PlayerController Object Reference")))

(fn `DestroyRandomCrates&FillRight`
  (locals (RandomCrate :type "/Game/Blueprints/WorldItems/Crates/BP_Crate Object Reference") (Crates :type "Array of /Game/Blueprints/WorldItems/Crates/BP_Crate Object Reference"))
  (bind _crates (`local.Crates`))
  (bind _outactors (`GameplayStatics.GetAllActorsOfClass` "/Game/Blueprints/WorldItems/Crates/BP_Crate.BP_Crate_C"))
  (set `local.Crates` _outactors)
  (for _ (range 1 (+ (`|GetArrayItem` (`self.CratesInfo`) 1) 1))
    (bind _output_get (set `local.RandomCrate` (`KismetArrayLibrary.Array_Random` _crates)))
    (`self.K2_DestroyActor` _output_get)
    (`KismetArrayLibrary.Array_RemoveItem` (`local.Crates`) _output_get)
    (`KismetSystemLibrary.PrintString` (`KismetStringLibrary.Conv_IntToString` (`KismetArrayLibrary.Array_Length` _crates)) true true (struct :`R` 1.0 :`G` 0.508 :`A` 1.0)))
  (bind _asgm_house (cast `/Game/ProjEng/Core/GameModes/GM_House` (`GameplayStatics.GetGameMode`)))
  (bind _returnvalue (`KismetSystemLibrary.MakeLiteralName` (`/Game/ProjEng/Core/GameModes/GM_House.RightCratesName` _asgm_house)))
  (bind _returnvalue_2 (`|GetDataTableRow` "/Game/Blueprints/WorldItems/Crates/DT_Crates.DT_Crates" _returnvalue)
    (:`then`
      (for _ (range 1 (+ (`|GetArrayItem` (`self.CratesInfo`)) 1))
        (bind _output_get_2 (set `local.RandomCrate` (`KismetArrayLibrary.Array_Random` (`local.Crates`))))
        (`/Game/Blueprints/WorldItems/Crates/BP_Crate.UpdateCrateInfo` _output_get_2 _returnvalue_2 _returnvalue)))))

(fn `SetContraband`
  (locals (L_Crates :type "Array of Object Object Reference")))

(fn `UpdateAddressesAndContraband`
  (locals (L_CurrentItemIndex :type Integer) (L_UnlockedHatch :type "/Game/ProjEng/Art/House/Hatch/BP_Hatch Object Reference"))
  (bind _addressnumber (`self.AddressNumber`))
  (bind _addressnumber_2 (`self.AddressNumber`))
  (bind (_outitem _outindex) (`KismetArrayLibrary.Array_Random` _addressnumber_2))
  (bind (_outitem_2 _outindex_2) (`KismetArrayLibrary.Array_Random` _addressnumber))
  (for _index (range 1 100)
    (`KismetArrayLibrary.Array_Add` (`self.AddressNumber`) (`KismetStringLibrary.Conv_StringToName` (`KismetStringLibrary.Conv_IntToString` _index))))
  ;[1 1 1] Add Contraband in Resources Array And delete it's address from list
  (bind _output_get (set `local.L_CurrentItemIndex` _outindex))
  (`KismetArrayLibrary.Array_Add` (`self.SResources`) (make `/Game/ProjEng/Art/House/Data/SResources` (struct) (`KismetStringLibrary.Conv_StringToName` (`KismetStringLibrary.Concat_StrStr` (`KismetStringLibrary.Conv_NameToString` (`KismetArrayLibrary.Array_Random` (`self.AddressName`))) " " (`KismetStringLibrary.Conv_NameToString` (`KismetArrayLibrary.Array_Random` (`self.AddressSecondName`))) " " (`KismetStringLibrary.Conv_NameToString` _outitem))) "NewEnumerator2"))
  (`KismetArrayLibrary.Array_Remove` _addressnumber_2 _output_get)
  ;[1 1 1] Fill Recources array with Addresses
  (bind _outactors (`GameplayStatics.GetAllActorsOfClass` null))
  (for _ (range (+ (+ (`KismetArrayLibrary.Array_Length` _outactors) 1) 1))
    (bind _output_get_2 (set `local.L_CurrentItemIndex` _outindex_2))
    (`KismetArrayLibrary.Array_Add` (`self.SResources`) (make `/Game/ProjEng/Art/House/Data/SResources` (struct) (`KismetStringLibrary.Conv_StringToName` (`KismetStringLibrary.Concat_StrStr` (`KismetStringLibrary.Conv_NameToString` (`KismetArrayLibrary.Array_Random` (`self.AddressName`))) " " (`KismetStringLibrary.Conv_NameToString` (`KismetArrayLibrary.Array_Random` (`self.AddressSecondName`))) " " (`KismetStringLibrary.Conv_NameToString` _outitem_2)))))
    (`KismetArrayLibrary.Array_Remove` _addressnumber _output_get_2))
  (return))

(fn `UserConstructionScript`)