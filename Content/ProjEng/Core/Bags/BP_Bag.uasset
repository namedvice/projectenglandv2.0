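; BP_Bag is a bag world item that the player carries on the SpineHandle socket.
; BeginPlay, after calling its parent, and OnInteract share one pickup sequence, so the bag also attaches itself at spawn.
; The sequence disables interaction, plays a zip sound, hands the bag to player 0's BPC_PlayerInventory via TakeWorldItemInHands, and adjusts mesh collision and physics.
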(event `self.ReceiveBeginPlay`
  (`parent.ReceiveBeginPlay`)
  (`self.DisableInteraction` :!label _label)
  (`PrimitiveComponent.SetCollisionEnabled` (`self.StaticMesh`) "QueryAndPhysics")
  (`GameplayStatics.PlaySound2D` "/Game/Sounds/Interactions/A_Zip1.A_Zip1" 1.0 2.0 0.0 null null)
  (`/Game/ProjEng/Data/Inventory/Components/BPC_PlayerInventory.TakeWorldItemInHands` (`self.GetComponentByClass` (`GameplayStatics.GetPlayerCharacter` 0) "/Game/ProjEng/Data/Inventory/Components/BPC_PlayerInventory.BPC_PlayerInventory_C") self "SpineHandle")
  (`PrimitiveComponent.SetSimulatePhysics` (`self.StaticMesh`) false))

(event `/Game/ProjEng/Data/Inventory/BPI_InventoryInteraction.OnInteract`
  (params (Actor :type "Actor Object Reference"))
  (goto _label))

(fn `UserConstructionScript`)